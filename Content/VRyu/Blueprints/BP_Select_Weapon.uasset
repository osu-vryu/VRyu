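; Weapon-selection challenge actor that completes when the player first grabs the katana held in its child BP_Sword.
; Construction applies optional mesh overrides to the sheath and decals.
; BeginPlay binds to the sword's first-grab event, which attaches the sheath to the katana, then destroys sheath and decals after a delay.
; It then calls OnChallengeBeat to report completion to the managing overlord.
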(event Custom|ExecuteDespawnSequence
  ;[0.15 0.15 0.15 0.5] When sword grabbed, run this custom event. This event is called from BP_Sword.
  (Development|PrintString "KATANA GRABBED")
  (bind _asbp_sword (Utilities|Casting|CastToBP_Sword (Variables|/Script/Engine.ChildActorComponent|GetChildActor (Variables|Default|GetSwordContainer)))
    (:then
      ;[0.15 0.15 0.15 0.5 16] After Cast, we now have reference to BP_Sword, so, grab Katana ref and do Attatch Comp to Comp, to bind the Local sheathe, to the Katana.
      (Transformation|AttachComponentToComponent (Variables|Default|GetSheathContainer) (Variables|/Game/VRyu/Blueprints/BP_Sword.BP_Sword_C|GetKatana _asbp_sword) "None" "KeepRelative" "KeepRelative" "KeepRelative" true)
      ;[0.15 0.15 0.15 0.5 16] Remove Meshes after 5s delay. TODO: dissolve material + user keystroke to begin rather than delay
      (Utilities|FlowControl|Delay 5.0)
      (Components|DestroyComponent (Variables|Default|GetSheathContainer))
      (Components|DestroyComponent (Variables|Default|Getdecals))
      ;[0.06125 0.06125 0.06125 1 16] indicates back to overlord that this is done.
      (Default|CallOnChallengeBeat))
    (:CastFailed
      (Development|PrintString "CAST FAILED"))))

(event EventBeginPlay
  (|CallParentFunction)
  ;[0.15 0.15 0.15 0.5] getter, now scoped as an actor. Then, casted to BP_sword, to ensure it's actually BP_sword, not just a generic 'actor', which is what UE presumes until explicitly Casted.
  (bind _asbp_sword (Utilities|Casting|CastToBP_Sword (Variables|/Script/Engine.ChildActorComponent|GetChildActor (Variables|Default|GetSwordContainer)))
    (:then
      ;[0.15 0.15 0.15 0.5] When sword grabbed, run this custom event. This event is called from BP_Sword.
      (EventDispatchers|BindEventtoOnSwordFirstGrabbed _asbp_sword (delegate Custom|ExecuteDespawnSequence)))
    (:CastFailed
      (Development|PrintString "ERR: Cast to BP_Sword FAILED in BP_Select_Weapon" true true "(R=1.000000,G=0.011239,B=0.346497,A=1.000000)" 5.0))))

(event Collision|EventActorBeginOverlap
  (params (OtherActor :type Actor%20Object%20Reference)))

(event EventTick
  (params (DeltaSeconds :type Float%20%28single-precision%29)))

(fn ConstructionScript
  (bind _sheathoverride (Variables|Default|GetSheathOverride))
  (bind _decaloverride (Variables|Default|GetDecalOverride))
  ;[0.15 0.15 0.15 0.5] On construction, check if SheathOverride was set (is valid), if it is, set it to the sheathe mesh.
  (Utilities|IsValid _sheathoverride
    (:Is%20Valid
      (Components|StaticMesh|SetStaticMesh (Variables|Default|GetSheathContainer) _sheathoverride))
    (:Is%20Not%20Valid
      _))
  ;[0.15 0.15 0.15 0.5] same process, but for decals
  (Utilities|IsValid _decaloverride
    (:Is%20Valid
      (Components|StaticMesh|SetStaticMesh (Variables|Default|Getdecals) _decaloverride))))