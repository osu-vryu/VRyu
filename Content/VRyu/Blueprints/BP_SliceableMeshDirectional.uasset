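; Sliceable mesh actor that only accepts slices made in a configured direction.
; ExtraSliceCheck compares strike velocity and slice normal against target directions within angle tolerances, optionally in the piece's local space.
; The normal match ignores sign, so a blade flipped 180 degrees passes, and zero vectors or 180-degree tolerances disable each test.
; Already-sliced pieces skip the check unless EnforceForRepeat is set; debug arrows and prints are switched off.
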(event EventBeginPlay
  (|CallParentFunction) ; This node is disabled and will not be called.\nDrag off pins to build functionality.
)

(event Collision|EventActorBeginOverlap
  (params (OtherActor :type Actor%20Object%20Reference))
  (|CallParentFunction OtherActor) ; This node is disabled and will not be called.\nDrag off pins to build functionality.
)

(event EventTick
  (params (DeltaSeconds :type Float%20%28single-precision%29))
  (|CallParentFunction DeltaSeconds) ; This node is disabled and will not be called.\nDrag off pins to build functionality.
)

(fn ConstructionScript
  (|CallParentFunction))

(fn ExtraSliceCheck
  (params (Piece :type S%20Sliceable%20Mesh%20Piece%20Structure%20%28by%20ref%29) (SlicePos :type Vector :default "0, 0, 0") (SliceNormal :type Vector :default "0, 0, 0") (StrikeVel :type Vector :default "0, 0, 0"))
  (bind _returnvalue (Transformation|GetActorLocation))
  (bind (_mesh _slicecount) (Utilities|Struct|BreakS_SliceableMeshPiece Piece))
  (bind _returnvalue_2 (Transformation|GetWorldTransform _mesh))
  (if (and (not (Variables|Default|GetEnforceForRepeat)) (> _slicecount 0))
    (return true)
    (else
      (if (not (Variables|Default|GetUseLocalDir))
        (LocalVariables|SetTransformedStrikeDir (Variables|Default|GetStrikeDir))
        (LocalVariables|SetTransformedNormal (Variables|Default|GetNormalDir))
        (else
          (LocalVariables|SetTransformedStrikeDir (Math|Transform|TransformDirection _returnvalue_2 (Variables|Default|GetStrikeDir)))
          (LocalVariables|SetTransformedNormal (Math|Transform|TransformDirection _returnvalue_2 (Variables|Default|GetNormalDir)))))
      (Utilities|FlowControl|Sequence
        (:then_0
          (CallFunction|DebugDrawDirVectorfromV "(R=1.000000,G=0.000000,B=0.000000,A=1.000000)" false _returnvalue (LocalVariables|GetTransformedStrikeDir))
          (CallFunction|DebugDrawDirVectorfromV "(R=0.000000,G=1.000000,B=0.122660,A=1.000000)" false _returnvalue (LocalVariables|GetTransformedNormal))
          (CallFunction|DebugDrawDirVectorfromV "(R=1.000000,G=0.869297,B=0.000000,A=1.000000)" false _returnvalue StrikeVel)
          (CallFunction|DebugDrawDirVectorfromV "(R=0.576631,G=0.000000,B=1.000000,A=1.000000)" false _returnvalue SliceNormal))
        (:then_1
          (CallFunction|DebugPrint false (Utilities|String|ToString(Text) (Utilities|Text|FormatText "Result of normal comparison: {comp}" (<= (Class|KismetMathLibrary|DegAcos (Math|Float|Absolute(Float) (CallFunction|Similarity (LocalVariables|GetTransformedNormal) SliceNormal))) (Variables|Default|GetNormalTolerance))))))
        (:then_2
          ;[0.15 0.15 0.15 0.5] Debug Angle Printing
          (CallFunction|DebugPrint false (Utilities|String|Append "strike angle: " (Utilities|String|ToString(Float) (Class|KismetMathLibrary|DegAcos (CallFunction|Similarity (LocalVariables|GetTransformedStrikeDir) StrikeVel)))))
          (CallFunction|DebugPrint false (Utilities|String|Append "normal angle: " (Utilities|String|ToString(Float) (Class|KismetMathLibrary|DegAcos (Math|Float|Absolute(Float) (CallFunction|Similarity (LocalVariables|GetTransformedNormal) SliceNormal))))))
          (return (and (or (or (>= (Variables|Default|GetStrikeTolerance) 1.8e+02) (Utilities|Operators|EqualEqual :A (LocalVariables|GetTransformedStrikeDir) :ErrorTolerance 0.0001)) (<= (Class|KismetMathLibrary|DegAcos (CallFunction|Similarity (LocalVariables|GetTransformedStrikeDir) StrikeVel)) (Variables|Default|GetStrikeTolerance))) (or (<= (Class|KismetMathLibrary|DegAcos (Math|Float|Absolute(Float) (CallFunction|Similarity (LocalVariables|GetTransformedNormal) SliceNormal))) (Variables|Default|GetNormalTolerance)) (or (Utilities|Operators|EqualEqual :A (LocalVariables|GetTransformedNormal) :ErrorTolerance 0.0001) (>= (Variables|Default|GetNormalTolerance) 1.8e+02))))))))))

(fn Similarity
  (params (a :type Vector) (b :type Vector))
  (return (Math|Vector|DotProduct (Math|Vector|Normalize a) (Math|Vector|Normalize b))))

(fn Dissimilarity
  (params (cosab :type Float%20%28double-precision%29))
  (return (- 1.0 cosab)))

(fn DebugDrawDirVectorfromV
  (params (color :type Linear%20Color%20Structure :default "(R=1.000000,G=0.000000,B=0.000000,A=1.000000)") (enabled :type Boolean) (v0 :type Vector) (vDir :type Vector))
  (if (and enabled (Variables|Default|GetbDebugMode))
    (Rendering|Debug|DrawDebugArrow v0 (+ (* vDir 1e+02) v0) 1.0 color 1e+01 2.0)))