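; BP_SliceableMeshLaunched is a sliceable mesh actor associated with a launcher, extending its parent's slicing behavior.
; On BeginPlay it binds to the first-slice event to increment the launcher's sliced count at the slice position.
; It also listens for piece hits, attempting to shrink any procedural mesh piece that strikes an actor carrying the delete tag.
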(event Custom|Event%20Notify%20Launcher
  (params (WorldPos :type Vector))
  (bind _associatedlauncher (Variables|Default|GetAssociatedLauncher))
  ;[0.15 0.15 0.15 0.5] Notify Launcher
  (if (Utilities|IsValid _associatedlauncher)
    (Default|IncrementSlicedCount _associatedlauncher WorldPos)))

(event Custom|OnPieceHit_Event
  (params (My%20Comp :type Primitive%20Component%20Object%20Reference) (Other :type Actor%20Object%20Reference) (Other%20Comp :type Primitive%20Component%20Object%20Reference) (Self%20Moved :type Boolean) (Hit%20Location :type Vector) (Hit%20Normal :type Vector) (Normal%20Impulse :type Vector) (Hit :type Hit%20Result%20Structure))
  ;[0.15 0.15 0.15 0.5] Check if mesh piece hit its delete plane/object
  (bind _asprocedural_mesh_component (Utilities|Casting|CastToProceduralMeshComponent My%20Comp))
  (if (Actor|ActorHasTag Other (Variables|Default|GetDeleteTag))
    (CallFunction|TryShrinkPiece _asprocedural_mesh_component)))

(event EventBeginPlay
  (|CallParentFunction)
  (Utilities|FlowControl|Sequence
    (:then_0
      ;[0.15 0.15 0.15 0.5] Notify Launcher
      (EventDispatchers|BindEventtoOnFirstSlice (delegate Custom|Event%20Notify%20Launcher)))
    (:then_1
      (EventDispatchers|AssignOnPieceHit (delegate Custom|OnPieceHit_Event)))))

(fn ConstructionScript
  (|CallParentFunction))