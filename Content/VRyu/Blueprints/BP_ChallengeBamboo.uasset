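; BP_ChallengeBamboo is a VR tameshigiri challenge where the player slices bamboo along shown directions through a sequence of stages.
; ChangeState shows the stage's arrow and spawns five shuffled-size directional sliceable stalks that enforce strike direction and blade normal.
; The first cut starts a countdown on Tick; cutting all five advances after a transition delay, while timeout respawns the stage.
; Floating widgets show progress or failure, and stage order can be randomized.
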(event OnComponentEndOverlap(DangerZone)
  (params (OverlappedComponent :type Primitive%20Component%20Object%20Reference) (OtherActor :type Actor%20Object%20Reference) (OtherComp :type Primitive%20Component%20Object%20Reference) (OtherBodyIndex :type Integer)))

(event EventBeginPlay
  (|CallParentFunction)
  (CallFunction|Init))

(event EventTick
  (params (DeltaSeconds :type Float%20%28single-precision%29))
  (|CallParentFunction DeltaSeconds)
  (if (Variables|Default|Get_ChallengeActive)
    (if (> (Variables|Default|GetTransitionTimer) 0.0)
      ;[0.15 0.15 0.15 0.5] Transition between bamboo stages
      (bind _output_get (Variables|Default|SetTransitionTimer (- (Variables|Default|GetTransitionTimer) DeltaSeconds)))
      (if (<= _output_get 0.0)
        (Variables|Default|SetTransitionTimer 0.0)
        (CallFunction|IncrementState))
      (else
        ;[0.15 0.15 0.15 0.5] Reset bamboo if not all sliced fast enough
        (if (Variables|Default|GetSliceBegun)
          (bind _output_get_2 (Variables|Default|SetResetTimer (- (Variables|Default|GetResetTimer) DeltaSeconds)))
          (if (<= _output_get_2 0.0)
            (CallFunction|ResetState)
            (CallFunction|SetCorrectnessIndicator "NewEnumerator2")))))))

(fn ConstructionScript)

(fn IncrementState
  (CallFunction|ChangeState (+ (Variables|Default|GetSliceIndex) 1)))

(fn ResetState
  (CallFunction|ChangeState (Variables|Default|GetSliceIndex)))

(fn ChangeState
  (params (NewIndex :type Integer))
  (bind _bambooorder (LocalVariables|GetBambooOrder))
  (bind _returnvalue (Utilities|Array|Length _bambooorder))
  (bind _returnvalue_2 (- _returnvalue 1))
  ;[0.15 0.15 0.15 0.5] Reset common variables
  (Variables|Default|SetSliceIndex NewIndex)
  (Variables|Default|SetBambooCut 0)
  (Variables|Default|SetResetTimer 0.0)
  (Variables|Default|SetTransitionTimer 0.0)
  (Variables|Default|SetSliceBegun false)
  (Utilities|FlowControl|Sequence
    (:then_0
      ;[0.15 0.15 0.15 0.5] Make current arrow invisble
      (if (Utilities|IsValid (Variables|Default|Get_CurrentArrow))
        (Rendering|SetVisibility (Variables|Default|Get_CurrentArrow) false false)))
    (:then_1
      (if (Utilities|IsCompleted)
        (Default|CallOnChallengeBeat)
        (else
          (Utilities|FlowControl|Sequence
            (:then_0
              ;[0.15 0.15 0.15 0.5] Destroy lingering bamboo
              (bind _arrayelement (Utilities|Array|ReverseforEachLoop (Variables|Default|GetBambooSliceables))
                (:LoopBody
                  (Utilities|IsValid _arrayelement
                    (:Is%20Valid
                      (Actor|DestroyActor _arrayelement))))
                (:Completed
                  (Utilities|Array|Clear (Variables|Default|GetBambooSliceables)))))
            (:then_1
              ;[0.15 0.15 0.15 0.5] Set visibility of and update direction helpers
              (Variables|Default|Set_CurrentArrow (.Direction (Utilities|Struct|BreakS_TameshigiriSliceParameter (Utilities|Array|Get(acopy) (Variables|Default|GetSliceParameters) (Variables|Default|GetSliceIndex)))))
              (Variables|Default|Set_CurrentNormal (.Normal (Utilities|Struct|BreakS_TameshigiriSliceParameter (Utilities|Array|Get(acopy) (Variables|Default|GetSliceParameters) (Variables|Default|GetSliceIndex)))))
              (Transformation|SetRelativeLocation (Transformation|GetAttachParent (Variables|Default|Get_CurrentArrow)) (Variables|/Script/Engine.SceneComponent|GetRelativeLocation (Variables|Default|GetSlice1)) false true)
              (Rendering|SetVisibility (Variables|Default|Get_CurrentArrow) true false))
            (:then_2
              ;[0.15 0.15 0.15 0.5] Spawn Bamboo Stalks
              (Utilities|FlowControl|Sequence
                (:then_0
                  (for _index (range 0 4)
                    (Utilities|Array|SetArrayElem (LocalVariables|GetBambooOrder) _index _index true))
                  (for _index_2 (range 0 _returnvalue_2)
                    (Utilities|Array|Swap (LocalVariables|GetBambooOrder) _index_2 (Math|Random|RandomIntegerinRange 0 _returnvalue_2))))
                (:then_1
                  (for (_array_element _array_index) (Components|GetChildrenComponents (Variables|Default|GetBambooHelpers) false)
                    (Utilities|FlowControl|Sequence
                      (:then_0
                        (switch int (Utilities|Array|Get(acopy) (LocalVariables|GetBambooOrder) _array_index)
                          (:0
                            (LocalVariables|SetBambooMesh "/Game/UsdAssets/SM_BambooSmallAlt.SM_BambooSmallAlt"))
                          (:1
                            (LocalVariables|SetBambooMesh "/Game/UsdAssets/SM_BambooSmall.SM_BambooSmall"))
                          (:2
                            (LocalVariables|SetBambooMesh "/Game/UsdAssets/SM_BambooMedium.SM_BambooMedium"))
                          (:3
                            (LocalVariables|SetBambooMesh "/Game/UsdAssets/SM_BambooLarge.SM_BambooLarge"))
                          (:4
                            (LocalVariables|SetBambooMesh "/Game/UsdAssets/SM_BambooExLarge.SM_BambooExLarge"))))
                      (:then_1
                        (bind _returnvalue_3 (Game|SpawnActorfromClass "/Game/VRyu/Blueprints/BP_SliceableMeshDirectional.BP_SliceableMeshDirectional_C" (Math|Transform|MakeTransform (.location (Transformation|GetWorldTransform _array_element)) "0, 0, 0" "1.000000,1.000000,1.100000") "Undefined" "MultiplyWithRoot" self (Math|Vector|GetForwardVector (Variables|Default|Get_CurrentArrow)) 6e+01 (Math|Vector|GetUpVector (Variables|Default|Get_CurrentNormal)) 35.0 true false (LocalVariables|GetBambooMesh) 25.0 3 0.35 0.35 1.0 "/Game/VRyu/Materials/M_BambooInsides.M_BambooInsides" "(R=1.000000,G=1.000000,B=1.000000,A=1.000000)" true 1.2e+02 1.25 true 0))
                        (EventDispatchers|BindEventtoOnFirstSlice _returnvalue_3 (EventDispatchers|CreateEvent :!event OnBambooSliced))
                        (Utilities|Array|Add (Variables|Default|GetBambooSliceables) _returnvalue_3)))))))))))))

(fn TransitiontoNextState
  (Variables|Default|SetTransitionTimer (Variables|Default|GetmaxTransitionTime))
  (CallFunction|SetCorrectnessIndicator "NewEnumerator0"))

(fn OnBambooSliced
  (params (WorldPos :type Vector))
  (if (Variables|Default|GetSliceBegun)
    _
    (else
      (Variables|Default|SetSliceBegun true)
      (Variables|Default|SetResetTimer (Variables|Default|GetmaxResetCountdown))))
  (Variables|Default|SetBambooCut (+ (Variables|Default|GetBambooCut) 1))
  (if (> (Variables|Default|GetBambooCut) 4)
    (CallFunction|TransitiontoNextState)))

(fn Init
  (bind _sliceparameters (Variables|Default|GetSliceParameters))
  (bind _returnvalue (Utilities|Array|Length _sliceparameters))
  (bind _returnvalue_2 (- _returnvalue 1))
  (Utilities|FlowControl|Sequence
    (:then_0
      ;[0.15 0.15 0.15 0.5] WHY CAN'T I JUST ASSIGN THESE AS A DEFAULT VALUE?!??!?!?!?!?!?
      (Utilities|FlowControl|Sequence
        (:then_0
          (Utilities|Array|Clear (Variables|Default|GetSliceParameters)))
        (:then_1
          (Utilities|Array|Add (Variables|Default|GetSliceParameters) (Utilities|Struct|MakeS_TameshigiriSliceParameter (Variables|Default|GetA1) (Variables|Default|GetN1))))
        (:then_2
          (Utilities|Array|Add (Variables|Default|GetSliceParameters) (Utilities|Struct|MakeS_TameshigiriSliceParameter (Variables|Default|GetA2) (Variables|Default|GetN2))))
        (:then_3
          (Utilities|Array|Add (Variables|Default|GetSliceParameters) (Utilities|Struct|MakeS_TameshigiriSliceParameter (Variables|Default|GetA3) (Variables|Default|GetN3))))
        (:then_4
          (Utilities|Array|Add (Variables|Default|GetSliceParameters) (Utilities|Struct|MakeS_TameshigiriSliceParameter (Variables|Default|GetA4) (Variables|Default|GetN4))))))
    (:then_1
      ;[0.15 0.15 0.15 0.5] Optionally randomize slice order
      (if (Variables|Default|GetRandomizeSliceOrder)
        (for _index (range 0 _returnvalue_2)
          (Utilities|Array|Swap (Variables|Default|GetSliceParameters) _index (Math|Random|RandomIntegerinRange 0 _returnvalue_2)))))
    (:then_2
      ;[0.15 0.15 0.15 0.5] Make all indicators invis by default
      (for _array_element (Variables|Default|GetSliceParameters)
        (Rendering|SetVisibility (.Direction (Utilities|Struct|BreakS_TameshigiriSliceParameter _array_element)) false false)))
    (:then_3
      ;[0.15 0.15 0.15 0.5] Reset simple vars
      (Variables|Default|SetTransitionTimer 0.0)
      (Variables|Default|SetResetTimer 0.0))))

(fn SetCorrectnessIndicator
  (params (correctness :type E_TameshigiriCorrectness%20Enum :default "NewEnumerator0"))
  (bind _length (Utilities|GetSequenceLength))
  (bind _sliceindex (Variables|Default|GetSliceIndex))
  (bind _correctnesswidgetloc (Variables|Default|GetCorrectnessWidgetLoc))
  (bind _returnvalue (Transformation|GetWorldLocation _correctnesswidgetloc))
  (bind _returnvalue_2 (Actor|GetActorOfClass "/Game/VRTemplate/Blueprints/VRPawn.VRPawn_C"))
  (Utilities|IsValid _returnvalue_2
    (:Is%20Valid
      (switch Utilities|FlowControl|Switch|SwitchonE_TameshigiriCorrectness correctness
        (:NewEnumerator0
          (Default|CreateNumberWidgetFloater _returnvalue_2 _returnvalue (Utilities|String|Append (Utilities|String|ToString(Integer) (+ _sliceindex 1)) "/" (Utilities|String|ToString(Integer) _length)) (Math|Float|MapRangeClamped (/ (Math|Conversions|ToFloat(Integer) _sliceindex) (Math|Conversions|ToFloat(Integer) (- _length 1))) 0.0 1.0 1.0 1.3) "(R=0.352941,G=1.000000,B=0.423529,A=1.000000)"))
        (:NewEnumerator2
          (Default|CreateNumberWidgetFloater _returnvalue_2 _returnvalue "X" 1.8 "(R=1.000000,G=0.050980,B=0.050980,A=1.000000)"))))))

(fn DebugPrint
  (params (bEnabled :type Boolean) (str :type String))
  (if (and bEnabled (Variables|Default|GetbDebugMode))
    (Development|PrintString (Utilities|String|ToString(Text) (Utilities|Text|FormatText "[BP_Bamboo_Enemy]: {String}" str)))))

(fn ResetChallenge
  (|CallParentFunction)
  (CallFunction|CleanupChallenge)
  (CallFunction|Init))

(fn CleanupChallenge
  (|CallParentFunction)
  (Utilities|FlowControl|Sequence
    (:then_0
      (bind _arrayelement (Utilities|Array|ReverseforEachLoop (Variables|Default|GetBambooSliceables))
        (:LoopBody
          (Utilities|IsValid _arrayelement
            (:Is%20Valid
              (Actor|DestroyActor _arrayelement))))))
    (:then_1
      (for _array_element (Variables|Default|GetSliceParameters)
        (Rendering|SetVisibility (.Direction (Utilities|Struct|BreakS_TameshigiriSliceParameter _array_element)) false false)))))

(fn StartChallenge
  (|CallParentFunction)
  (CallFunction|ChangeState)
  (Variables|Default|Set_ChallengeActive true))