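; Teacup challenge for a VR game, built on a parent challenge class, that completes when the VR pawn enters its collision volume.
; Starting it turns on sprinkler and video mist systems, then Tick polls for overlapping pawns.
; Despite its name, ShowCredits only marks completion and calls OnChallengeBeat.
; Reset deactivates both systems and clears the state, though CanBeReset always returns false.
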(event EventBeginPlay
  (|CallParentFunction)
  (Variables|Default|SetIsComplete false)
  (Variables|Default|SetChallengeActive false))

(event Collision|EventActorBeginOverlap
  (params (OtherActor :type Actor%20Object%20Reference))
  (|CallParentFunction OtherActor))

(event EventTick
  (params (DeltaSeconds :type Float%20%28single-precision%29))
  (|CallParentFunction DeltaSeconds)
  (if (Variables|Default|GetChallengeActive)
    (if (not (Variables|Default|GetIsComplete))
      (bind _array_element (Utilities|Array|ForEachLoopwithBreak (Collision|GetOverlappingActors (Variables|Default|GetCollision) "/Game/VRTemplate/Blueprints/VRPawn.VRPawn_C" :!class /Script/Engine.PrimitiveComponent) :!label _label)
        (:LoopBody
          (Utilities|IsValid _array_element
            (:Is%20Valid
              (CallFunction|ShowCredits)
              (goto _label Break))))))))

(fn ConstructionScript)

(fn ShowCredits
  (Utilities|FlowControl|Sequence
    (:then_0
      (Variables|Default|SetIsComplete true))
    (:then_1
      (Default|CallOnChallengeBeat))))

(fn HideCredits
  (Variables|Default|SetIsComplete false))

(fn DebugPrint
  (params (bEnabled :type Boolean) (str :type String))
  (if (and bEnabled (Variables|Default|GetbDebugMode))
    (Development|PrintString (Utilities|String|ToString(Text) (Utilities|Text|FormatText "[BP_Teacup]: {String}" str)))))

(fn DebugInit)

(fn CleanupChallenge
  (|CallParentFunction)
  (Components|Activation|Deactivate (Variables|Default|GetSmallSprinkler_System))
  (Components|Activation|Deactivate (Variables|Default|GetVideo_Mist_System)))

(fn ResetChallenge
  (|CallParentFunction)
  (CallFunction|CleanupChallenge)
  (CallFunction|HideCredits)
  (Variables|Default|SetChallengeActive false))

(fn StartChallenge
  (|CallParentFunction)
  (Variables|Default|SetChallengeActive true)
  (Components|Activation|Activate (Variables|Default|GetSmallSprinkler_System) true)
  (Components|Activation|Activate (Variables|Default|GetVideo_Mist_System) true))

(fn CanbeReset
  (return false))