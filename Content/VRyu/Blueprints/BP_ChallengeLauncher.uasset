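; VR slicing challenge that flings sliceable objects from the actor until enough have been sliced, built on a parent challenge class.
; While active, Tick prunes destroyed objects and spawns new ones on a random timer, launching their physics pieces along a randomized cone direction with optional random spin.
; IncrementSlicedCount shows a growing progress floater through the VRPawn and ends the challenge at the target count.
; Start, reset and cleanup overrides manage launching and destroy spawned objects.
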(event EventBeginPlay
  (|CallParentFunction))

(event EventTick
  (params (DeltaSeconds :type Float%20%28single-precision%29))
  (bind __objects (Variables|Default|Get_objects))
  (bind _returnvalue (Utilities|Array|Length __objects))
  (bind _returnvalue_2 (- _returnvalue 1))
  (|CallParentFunction DeltaSeconds)
  (if (Variables|Default|Get_active)
    (Utilities|FlowControl|Sequence
      (:then_0
        ;[0.15 0.15 0.15 0.5] Forget deleted sliceables
        (for _index (range 0 _returnvalue_2)
          (if (not (Utilities|IsValid (Utilities|Array|Get(acopy) (Variables|Default|Get_objects) (- _returnvalue_2 _index))))
            (Utilities|Array|RemoveIndex (Variables|Default|Get_objects) (- _returnvalue_2 _index)))))
      (:then_1
        ;[0.15 0.15 0.15 0.5] Launch new objects on a timer
        (bind _output_get (Variables|Default|Set_Timer_0 (- (Variables|Default|Get_Timer_0) DeltaSeconds)))
        (if (<= _output_get 0.0)
          (CallFunction|LaunchObject)
          (CallFunction|ResetTimer))))))

(fn ConstructionScript)

(fn StartLaunching
  (CallFunction|ResetLaunching)
  (Variables|Default|Set_active true))

(fn ResetLaunching
  (Utilities|IsValid (Game|GetGameState)
    (:Is%20Valid
      (if (> (Class|GameplayStatics|GetNumPlayerControllers) 0)
        (Utilities|FlowControl|Sequence
          (:then_0
            ;[0.15 0.15 0.15 0.5] Delete existing launched objects
            (for _array_element (Variables|Default|Get_objects)
              (Actor|DestroyActor _array_element)))
          (:then_1
            ;[0.15 0.15 0.15 0.5] Reset Variables
            (Utilities|Array|Clear (Variables|Default|Get_objects))
            (Variables|Default|Set_slicedCount 0)
            (Variables|Default|Set_Timer_0 0.0)
            (Variables|Default|Set_active false)))))))

(fn FinishLaunching
  (Variables|Default|Set_active false)
  (Default|CallOnChallengeBeat))

(fn CalculateLaunchDir
  (bind _dirrandvert (Variables|Default|GetDirRandVert))
  (bind _dirrandhoriz (Variables|Default|GetDirRandHoriz))
  (return (Math|Vector|Normalize (Math|Vector|RotateVectorAroundAxis (Math|Vector|RotateVectorAroundAxis (Math|Transform|TransformDirection (Transformation|GetWorldTransform (Variables|Default|GetDefaultSceneRoot)) (Variables|Default|GetDirection)) (Math|Random|RandomFloatinRange _dirrandhoriz (* _dirrandhoriz -1.0)) "0.000000,0.000000,1.000000") (Math|Random|RandomFloatinRange _dirrandvert (* _dirrandvert -1.0)) (Math|Vector|CrossProduct (Variables|Default|GetDirection) "0.000000,0.000000,1.000000")))))

(fn ResetTimer
  (bind _timerinterval (Variables|Default|GetTimerInterval))
  (bind (_min _max) (Utilities|Struct|BreakFloatInterval _timerinterval))
  (Variables|Default|Set_Timer_0 (Math|Random|RandomFloatinRange _min _max))
  (return))

(fn LaunchObject
  (bind _self self)
  (bind _rotvel (Variables|Default|GetRotVel))
  (bind _returnvalue (* _rotvel -1.0))
  (bind _normed_dir (CallFunction|CalculateLaunchDir))
  (bind _output_get (LocalVariables|SetDir _normed_dir))
  (if (Variables|Default|GetRandomizeRotation)
    (LocalVariables|SetRotation (Math|Rotator|MakeRotator (Math|Random|RandomFloatinRange 0.0 3.6e+02) (Math|Random|RandomFloatinRange 0.0 3.6e+02) (Math|Random|RandomFloatinRange 0.0 3.6e+02)))
    (else
      (LocalVariables|SetRotation (Math|Rotator|FindLookatRotation (Class|KismetMathLibrary|VectorForward) _output_get))))
  (bind _returnvalue_2 (Game|SpawnActorfromClass (Variables|Default|GetObjectType) (Math|Transform|MakeTransform (.Location (Math|Transform|BreakTransform (Transformation|GetActorTransform))) (LocalVariables|GetRotation)) "AdjustIfPossibleButAlwaysSpawn" "MultiplyWithRoot" _self "Floor" _self 0 6e+01 3 0.25 0.0 1.25 "/Game/VRyu/Materials/M_WatermelonInsides.M_WatermelonInsides" "(R=0.749020,G=0.007843,B=0.015686,A=1.000000)" true 45.0 1.25 true 0))
  (Utilities|Array|Add (Variables|Default|Get_objects) _returnvalue_2)
  (Utilities|FlowControl|Sequence
    (:then_0
      ;[0.15 0.15 0.15 0.5] Calc random ang vel
      (LocalVariables|SetRandAngVel (Math|Vector|MakeVector (Math|Random|RandomFloatinRange _returnvalue _rotvel) (Math|Random|RandomFloatinRange _returnvalue _rotvel) (Math|Random|RandomFloatinRange _returnvalue _rotvel))))
    (:then_1
      ;[0.15 0.15 0.15 0.5] Fling the generated piece!
      (for _array_element (Variables|/Game/VRyu/Blueprints/BP_SliceableMesh.BP_SliceableMesh_C|GetPieces _returnvalue_2)
        (Collision|SetCollisionEnabled (.Mesh (Utilities|Struct|BreakS_SliceableMeshPiece _array_element)) "QueryAndPhysics")
        (Physics|SetSimulatePhysics (.Mesh (Utilities|Struct|BreakS_SliceableMeshPiece _array_element)) true)
        (Physics|SetPhysicsLinearVelocity (.Mesh (Utilities|Struct|BreakS_SliceableMeshPiece _array_element)) (* (LocalVariables|GetDir) (Variables|Default|GetVel)) false "None")
        (if (Variables|Default|GetRandomizeRotation)
          (Class|PrimitiveComponent|SetPhysicsAngularVelocityinDegrees (.Mesh (Utilities|Struct|BreakS_SliceableMeshPiece _array_element)) (LocalVariables|GetRandAngVel) false "None"))))))

(fn IncrementSlicedCount
  (params (Location :type Vector))
  (bind _objectcount (Variables|Default|GetObjectCount))
  (if (Variables|Default|Get_active)
    (Utilities|FlowControl|Sequence
      (:then_0
        ;[0.15 0.15 0.15 0.5] Increment Count
        (Variables|Default|Set_slicedCount (+ (Variables|Default|Get_slicedCount) 1)))
      (:then_1
        ;[0.15 0.15 0.15 0.5] Create Visual Counter
        (bind _returnvalue (Actor|GetActorOfClass "/Game/VRTemplate/Blueprints/VRPawn.VRPawn_C"))
        (Utilities|IsValid _returnvalue
          (:Is%20Valid
            (Default|CreateNumberWidgetFloater _returnvalue (+ Location (Variables|Default|GetCounterWidgetOffset)) (Utilities|String|Append (Utilities|String|ToString(Integer) (Variables|Default|Get_slicedCount)) "/" (Utilities|String|ToString(Integer) _objectcount)) (Math|Float|MapRangeClamped (/ (Math|Conversions|ToFloat(Integer) (- (Variables|Default|Get_slicedCount) 1)) (Math|Conversions|ToFloat(Integer) (- _objectcount 1))) 0.0 1.0 0.8 1.6) "(R=0.352941,G=1.000000,B=0.423529,A=1.000000)"))))
      (:then_2
        ;[0.15 0.15 0.15 0.5] Possibly Move On
        (if (>= (Variables|Default|Get_slicedCount) (Variables|Default|GetObjectCount))
          (CallFunction|FinishLaunching))))))

(fn DebugPrint
  (params (bEnabled :type Boolean) (str :type String))
  (if (and bEnabled (Variables|Default|GetbDebugMode))
    (Development|PrintString (Utilities|String|ToString(Text) (Utilities|Text|FormatText "[BP_ObjectLauncher]: {String}" str)))))

(fn DebugInit)

(fn ResetChallenge
  (|CallParentFunction)
  (CallFunction|CleanupChallenge)
  (CallFunction|ResetLaunching))

(fn CleanupChallenge
  (|CallParentFunction)
  (Utilities|FlowControl|Sequence
    (:then_0
      (bind _arrayelement (Utilities|Array|ReverseforEachLoop (Variables|Default|Get_objects))
        (:LoopBody
          (Utilities|IsValid _arrayelement
            (:Is%20Valid
              (Actor|DestroyActor _arrayelement))))))
    (:then_1
      (Utilities|Array|Clear (Variables|Default|Get_objects))
      (Variables|Default|Set_active false))))

(fn StartChallenge
  (Utilities|IsValid (Game|GetGameState)
    (:Is%20Valid
      (if (> (Class|GameplayStatics|GetNumPlayerControllers) 0)
        (|CallParentFunction)
        (CallFunction|StartLaunching)))))