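; Sliceable hanging lantern that sways procedurally on a cable until cut, then resets after a delay.
; Builds on a parent sliceable class, tying the cable to each new unsliced procedural mesh and releasing it on first slice.
; TrySlice intercepts cable hits to sever the cable, drop the lantern with physics and play a sound.
; Tick drives the summed-sine sway and the reset timer, which pauses while pieces are frozen.
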(event Custom|TieCableToNewProcMesh
  (params (StaticMesh :type Static%20Mesh%20Component%20Object%20Reference) (ProcMesh :type Procedural%20Mesh%20Component%20Object%20Reference) (NewPieceIndex :type Integer))
  (Variables|Default|Set_CurrentOriginalPiece ProcMesh)
  (CallFunction|TieCabletoProcMesh ProcMesh))

(event Custom|OnFirstSlicedPiece
  (params (Piece :type Integer) (OtherHalf :type Integer))
  (Utilities|FlowControl|Sequence
    (:then_0
      (Variables|Default|Set_ResetTimer (Variables|Default|GetResetTime)))
    (:then_1
      (CallFunction|UntieCablefromProcMesh (.Mesh (Utilities|Struct|BreakS_SliceableMeshPiece (Utilities|Array|Get(acopy) (Variables|Default|GetPieces) Piece))) false))))

(event EventBeginPlay
  (bind _cable (Variables|Default|GetCable))
  (bind _endlocation (Variables|/Script/CableComponent.CableComponent|GetEndLocation _cable))
  (bind (_x _y) (Math|Vector|BreakVector _endlocation))
  (Utilities|FlowControl|Sequence
    (:then_0
      (Variables|Default|Set_OrginalCableLength (Variables|/Script/CableComponent.CableComponent|GetCableLength (Variables|Default|GetCable)))
      (Variables|Default|Set_OriginalRot (Variables|/Script/Engine.SceneComponent|GetRelativeRotation (Variables|Default|GetCable)))
      (Variables|Default|Set_OriginalCableAttachLateralDist (Math|Vector|VectorLength (Math|Vector|MakeVector _x _y 0.0))))
    (:then_1
      (EventDispatchers|BindEventtoOnCreateUnslicedProcMesh (delegate Custom|TieCableToNewProcMesh))
      (EventDispatchers|BindEventtoOnFirstSliceOfPiece (delegate Custom|OnFirstSlicedPiece))
      (|CallParentFunction))))

(event Collision|EventActorBeginOverlap
  (params (OtherActor :type Actor%20Object%20Reference))
  (|CallParentFunction OtherActor) ; This node is disabled and will not be called.\nDrag off pins to build functionality.
)

(event EventTick
  (params (DeltaSeconds :type Float%20%28single-precision%29))
  (bind _pieces (Variables|Default|GetPieces))
  (bind __currentoriginalpiece (Variables|Default|Get_CurrentOriginalPiece))
  (bind _index (CallFunction|GetPieceIndex __currentoriginalpiece))
  (bind _output (Utilities|Array|Get(acopy) _pieces _index))
  (bind (_mesh _slicecount) (Utilities|Struct|BreakS_SliceableMeshPiece _output))
  (|CallParentFunction DeltaSeconds)
  (if (Variables|Default|Get_Enabled)
    (Variables|Default|Set_FirstFrame false)
    (Utilities|FlowControl|Sequence
      (:then_0
        ;[0.15 0.15 0.15 0.5] Spinning before cut
        (if (and (not (Variables|Default|Get_CableBeenCut)) (Utilities|Array|IsValidIndex (Variables|Default|GetPieces) _index))
          (if (<= _slicecount 0)
            (Transformation|SetRelativeRotation _mesh (Math|Rotator|CombineRotators (Variables|Default|Get_OriginalRot) (CallFunction|SpinningFunc (Utilities|Time|GetGameTimeinSeconds))) false false))))
      (:then_1
        ;[0.15 0.15 0.15 0.5] Reset timer
        (if (> (Variables|Default|Get_ResetTimer) 0.0)
          (if (not (CallFunction|HasFrozenPieces))
            (Variables|Default|Set_ResetTimer (- (Variables|Default|Get_ResetTimer) DeltaSeconds))
            (if (<= (Variables|Default|Get_ResetTimer) 0.0)
              (Default|ResetSliceable self true false)
              (Variables|Default|Set_ResetTimer 0.0))))))))

(fn ConstructionScript
  (|CallParentFunction))

(fn TrySlice
  (params (SlicePos :type Vector :default "0, 0, 0") (SliceNormal :type Vector :default "0, 0, 0") (StrikeVel :type Vector :default "0, 0, 0") (HitComponent :type Primitive%20Component%20Object%20Reference))
  (bind _pieces (Variables|Default|GetPieces))
  (bind __currentoriginalpiece (Variables|Default|Get_CurrentOriginalPiece))
  (bind _cable (Variables|Default|GetCable))
  (bind _index (CallFunction|GetPieceIndex __currentoriginalpiece))
  (bind _output (Utilities|Array|Get(acopy) _pieces _index))
  (bind (_mesh _slicecount) (Utilities|Struct|BreakS_SliceableMeshPiece _output))
  (if (Variables|Default|Get_Enabled)
    (if (or (== HitComponent (Variables|Default|GetCable)) (== HitComponent (Variables|Default|GetCableCollision)))
      (if (not (Variables|Default|Get_CableBeenCut))
        (if (Utilities|Array|IsValidIndex (Variables|Default|GetPieces) _index)
          (if (<= _slicecount 0)
            (Variables|Default|Set_CableBeenCut true)
            (Utilities|FlowControl|Sequence
              (:then_0
                ;[0.15 0.15 0.15 0.5] Sever/shorten cable
                (Variables|/Script/CableComponent.CableComponent|SetCableLength _cable (* (Variables|/Script/CableComponent.CableComponent|GetCableLength _cable) 0.85))
                (CallFunction|UntieCablefromProcMesh _mesh true)
                (Physics|SetSimulatePhysics _mesh true)
                (Utilities|Struct|SetmembersinS_SliceableMeshPiece (Utilities|Array|Get(acopy) (Variables|Default|GetPieces) (CallFunction|GetPieceIndex (Variables|Default|Get_CurrentOriginalPiece))) (Utilities|Time|GetGameTimeinSeconds) true))
              (:then_1
                ;[0.15 0.15 0.15 0.5] Play sound
                (bind _asbp_vryu_game_instance (Utilities|Casting|CastToBP_VRyuGameInstance (Game|GetGameInstance)))
                (Default|PlayManagedSound _asbp_vryu_game_instance "NewEnumerator12" (Transformation|GetActorLocation) (Math|Random|RandomFloatinRange 0.875 1.125)))
              (:then_2
                ;[0.15 0.15 0.15 0.5] Allow it to despawn/reset now!
                (Variables|Default|Set_ResetTimer (Variables|Default|GetResetTime)))))))
      (else
        (bind _sliceresult (|CallParentFunction SlicePos SliceNormal StrikeVel HitComponent))
        (return _sliceresult)))))

(fn TieCabletoProcMesh
  (params (ProcMesh :type Procedural%20Mesh%20Component%20Object%20Reference))
  (Variables|/Script/CableComponent.CableComponent|SetCableLength (Variables|Default|GetCable) (Variables|Default|Get_OrginalCableLength))
  (Variables|/Script/CableComponent.CableComponent|SetbAttachEnd (Variables|Default|GetCable) true)
  (Class|CableComponent|SetAttachEndtoComponent (Variables|Default|GetCable) ProcMesh "None")
  (Variables|Default|Set_CableBeenCut false)
  (Rendering|SetVisibility (Variables|Default|GetCable) true false))

(fn UntieCablefromProcMesh
  (params (ProcMesh :type Procedural%20Mesh%20Component%20Object%20Reference) (Force :type Boolean))
  (bind _cable (Variables|Default|GetCable))
  (if (or (== (Components|GetOwner ProcMesh) (Class|CableComponent|GetAttachedActor (Variables|Default|GetCable))) Force)
    (Utilities|FlowControl|Sequence
      (:then_0
        (if (Variables|Default|GetMakeUnattachedCableInvis)
          (Rendering|SetVisibility (Variables|Default|GetCable) false false)))
      (:then_1
        (Class|CableComponent|SetAttachEndtoComponent _cable 0 "None")
        (Variables|/Script/CableComponent.CableComponent|SetbAttachEnd _cable false)))))

(fn SpinningFunc
  (params (Time :type Float%20%28double-precision%29))
  (return (Math|Rotator|MakeRotator (Class|KismetMathLibrary|FWrap (+ (* (Math|Trig|Sin(Degrees) (+ (* Time 35.09235) 24.64737)) 0.585) (* (Math|Trig|Cos(Degrees) (+ (* Time 20.542366) 27.049861)) 0.975)) 0.0 3.6e+02) (Class|KismetMathLibrary|FWrap (+ (* (Math|Trig|Sin(Degrees) (+ (* Time 33.902835) 824.634677)) 0.39) (* (Math|Trig|Cos(Degrees) (+ (* Time 21.238707) 1.590782)) 0.78)) 0.0 3.6e+02) (Class|KismetMathLibrary|FWrap (+ (* (Math|Trig|Sin(Degrees) (+ (* Time 16.3677) 2.35674)) 28.0) (* (Math|Trig|Cos(Degrees) (+ (* Time 10.5324) 293.536527)) 48.0) (* (Math|Trig|Sin(Degrees) (+ (* Time 5.2478) 23.6478)) 6e+01)) 0.0 3.6e+02))))

(fn Enable
  (Variables|Default|Set_Enabled true)
  (CallFunction|CreateUnslicedPiecefromStaticMesh)
  (Rendering|SetVisibility (Variables|Default|GetCable) true false))

(fn Disable
  (Variables|Default|Set_Enabled false)
  (Utilities|FlowControl|Sequence
    (:then_0
      (if (Variables|Default|Get_FirstFrame)
        (CallFunction|DeleteAllPieces false)
        (else
          (CallFunction|ShrinkAll))))
    (:then_1
      (Rendering|SetVisibility (Variables|Default|GetCable) false false))))