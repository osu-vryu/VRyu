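; Abstract base for challenges, tracking a beaten, resolved and cleanup lifecycle.
; Beat and resolved dispatchers set state flags and restart a shared timer on Tick, which fires resolution after ResolutionDelay and CleanupChallenge after CleanupDelay.
; A delay of zero or less disables that automatic step.
; Start and cleanup are empty stubs, reset clears the state, and CanBeReset returns true by default.
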(event Custom|ResolutionInitiator
  ;[0.15 0.15 0.15 0.5] Beat/resolution listener
  (if (not (Variables|Default|Get_HasBeenBeat))
    (Variables|Default|Set_Timer 0.0)
    (Variables|Default|Set_HasBeenBeat true)
    (Variables|Default|Set_HasBeenResolved false)))

(event Custom|CleanupInitiator
  ;[0.15 0.15 0.15 0.5] Resolution/cleanup listener
  (if (not (Variables|Default|Get_HasBeenResolved))
    (Variables|Default|Set_Timer 0.0)
    (Variables|Default|Set_HasBeenBeat true)
    (Variables|Default|Set_HasBeenResolved true)))

(event EventBeginPlay
  (Utilities|FlowControl|Sequence
    (:then_0
      ;[0.15 0.15 0.15 0.5] Beat/resolution listener
      (EventDispatchers|BindEventtoOnChallengeBeat (delegate Custom|ResolutionInitiator)))
    (:then_1
      ;[0.15 0.15 0.15 0.5] Resolution/cleanup listener
      (EventDispatchers|AssignOnChallengeResolved (delegate Custom|CleanupInitiator)))))

(event EventTick
  (params (DeltaSeconds :type Float%20%28single-precision%29))
  (bind _resolutiondelay (Variables|Default|GetResolutionDelay))
  (bind _cleanupdelay (Variables|Default|GetCleanupDelay))
  (if (Variables|Default|Get_HasBeenBeat)
    (if (Variables|Default|Get_HasBeenResolved)
      ;[0.15 0.15 0.15 0.5] Cleanup after resolution (if enabled)
      (if (and (< (Variables|Default|Get_Timer) _cleanupdelay) (> _cleanupdelay 0.0))
        (bind _output_get (Variables|Default|Set_Timer (+ (Variables|Default|Get_Timer) DeltaSeconds)))
        (if (>= _output_get (Variables|Default|GetCleanupDelay))
          (Variables|Default|Set_Timer (Variables|Default|GetCleanupDelay))
          (CallFunction|CleanupChallenge)))
      (else
        ;[0.15 0.15 0.15 0.5] Resolve after beating
        (if (and (< (Variables|Default|Get_Timer) _resolutiondelay) (> _resolutiondelay 0.0))
          (bind _output_get_2 (Variables|Default|Set_Timer (+ (Variables|Default|Get_Timer) DeltaSeconds)))
          (if (>= _output_get_2 (Variables|Default|GetResolutionDelay))
            (Variables|Default|Set_Timer (Variables|Default|GetResolutionDelay))
            (Default|CallOnChallengeResolved)))))))

(fn ConstructionScript)

(fn StartChallenge)

(fn ResetChallenge
  (Variables|Default|Set_HasBeenBeat false)
  (Variables|Default|Set_HasBeenResolved false)
  (Variables|Default|Set_Timer 0.0))

(fn CleanupChallenge)

(fn HasBeenBeat
  (return (Variables|Default|Get_HasBeenBeat)))

(fn HasBeenResolved
  (return (Variables|Default|Get_HasBeenResolved)))

(fn CanbeReset
  (return true))