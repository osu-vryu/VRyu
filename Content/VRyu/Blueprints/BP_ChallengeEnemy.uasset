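; Combat challenge that spawns enemies to chase the player and is beaten once all of them are defeated.
; StartChallenge spawns three enemies at marker components when IsLevel2 is set, otherwise one with a floating "Block or Attack!" prompt on the VR pawn.
; Each enemy's defeat event feeds a counter that fires OnChallengeBeat once it reaches the spawn count.
; Reset destroys the tracked enemies and clears the counters.
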(event EventBeginPlay
  (|CallParentFunction))

(event Collision|EventActorBeginOverlap
  (params (OtherActor :type Actor%20Object%20Reference))
  (|CallParentFunction OtherActor) ; This node is disabled and will not be called.\nDrag off pins to build functionality.
)

(event EventTick
  (params (DeltaSeconds :type Float%20%28single-precision%29))
  (|CallParentFunction DeltaSeconds))

(fn ConstructionScript
  (|CallParentFunction))

(fn SpawnEnemy
  (params (Loc :type Vector) (Rot :type Rotator) (SpawnDialog :type Boolean))
  (Utilities|FlowControl|Sequence
    (:then_0
      (if SpawnDialog
        (bind _returnvalue (Actor|GetActorOfClass "/Game/VRTemplate/Blueprints/VRPawn.VRPawn_C"))
        (Default|CreateDialogWidgetFloater _returnvalue (+ Loc "0.000000,0.000000,210.000000") 5.0 "Block or Attack!" 1.0 "(R=1.000000,G=1.000000,B=1.000000,A=1.000000)")))
    (:then_1
      (bind _returnvalue_2 (Game|SpawnActorfromClass "/Game/VRyu/Blueprints/BP_Enemy.BP_Enemy_C" (Math|Transform|MakeTransform Loc Rot) "AdjustIfPossibleButAlwaysSpawn" "MultiplyWithRoot" self 0))
      (Utilities|Array|Add (Variables|Default|Get_SpawnedEnemies) _returnvalue_2)
      (EventDispatchers|BindEventtoOnEnemyDefeated _returnvalue_2 (EventDispatchers|CreateEvent :!event OnDefeatEnemy))
      (Default|ChasePlayer _returnvalue_2))
    (:then_2
      (Variables|Default|Set_EnemyCount (+ (Variables|Default|Get_EnemyCount) 1)))))

(fn OnDefeatEnemy
  (params (Enemy :type BP%20Enemy%20Object%20Reference))
  (EventDispatchers|UnbindallEventsfromOnEnemyDefeated Enemy)
  (bind _output_get (Variables|Default|Set_EnemiesDefeated (+ (Variables|Default|Get_EnemiesDefeated) 1)))
  (if (>= _output_get (Variables|Default|Get_EnemyCount))
    (if (not (Variables|Default|GetDefeated))
      (Variables|Default|SetDefeated true)
      (Default|CallOnChallengeBeat))))

(fn ResetChallenge
  (|CallParentFunction)
  (CallFunction|CleanupChallenge)
  (Variables|Default|SetDefeated false)
  (Variables|Default|Set_EnemiesDefeated 0)
  (Variables|Default|Set_EnemyCount 0))

(fn StartChallenge
  (|CallParentFunction)
  (if (Variables|Default|GetIsLevel2)
    (CallFunction|SpawnEnemy (Transformation|GetWorldLocation (Variables|Default|GetEnemy%20Loc1)) (Transformation|GetWorldRotation (Variables|Default|GetEnemy%20Rot1)) false)
    (CallFunction|SpawnEnemy (Transformation|GetWorldLocation (Variables|Default|GetEnemy%20Loc2)) (Transformation|GetWorldRotation (Variables|Default|GetEnemy%20Rot2)) false)
    (CallFunction|SpawnEnemy (Transformation|GetWorldLocation (Variables|Default|GetEnemy%20Loc3)) (Transformation|GetWorldRotation (Variables|Default|GetEnemy%20Rot3)) false)
    (else
      (CallFunction|SpawnEnemy (Transformation|GetWorldLocation (Variables|Default|GetEnemy%20Loc)) (Transformation|GetWorldRotation (Variables|Default|GetEnemy%20Rot)) true))))

(fn CleanupChallenge
  (|CallParentFunction)
  (for _array_element (Variables|Default|Get_SpawnedEnemies)
    (Utilities|IsValid _array_element
      (:Is%20Valid
        (Actor|DestroyActor _array_element))))
  (Utilities|Array|Clear (Variables|Default|Get_SpawnedEnemies)))