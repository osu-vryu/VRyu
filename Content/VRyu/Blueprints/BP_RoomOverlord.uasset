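; BP_RoomOverlord is the game's state machine, sequencing a VR run from main title through weapon selection, slicing and enemy challenges, and a tea room to the end menu.
; ChangeState unbinds old challenges, then either initializes immediately or advances BP_RailManager and waits for the pawn's rail movement to complete.
; InitState binds and starts each state's challenges, and handles menus, the slicing lantern and sword removal.
; It also supports skipping and restarting challenges.
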(event Custom|OnVictory
  (CallFunction|IncrementState false))

(event Custom|OnRailsComplete
  (if (Variables|Default|GetIsTransitioning)
    (Variables|Default|SetIsTransitioning false)
    (CallFunction|InitState)))

(event EventBeginPlay
  (Utilities|FlowControl|Sequence
    (:then_0
      (bind _returnvalue (Actor|GetActorOfClass "/Game/VRyu/Blueprints/BP_RailManager.BP_RailManager_C"))
      (Variables|Default|Set_RailManager _returnvalue))
    (:then_1
      (bind _returnvalue_2 (Actor|GetActorOfClass "/Game/VRTemplate/Blueprints/VRPawn.VRPawn_C"))
      (bind _output_get (Variables|Default|Set_VRPawn _returnvalue_2))
      (Utilities|IsValid _output_get
        (:Is%20Valid
          (EventDispatchers|BindEventtoOnRailsMovementComplete _output_get (delegate Custom|OnRailsComplete)))
        (:Is%20Not%20Valid
          (Development|PrintString "ERROR: no player pawn detected, cannot bind movement event" true true "(R=1.000000,G=0.000000,B=0.000000,A=1.000000)" 4.0))))
    (:then_2
      (CallFunction|ChangeState "NewEnumerator0" false))))

(event Collision|EventActorBeginOverlap
  (params (OtherActor :type Actor%20Object%20Reference)))

(event EventTick
  (params (DeltaSeconds :type Float%20%28single-precision%29))
  (if (Variables|Default|Get_IncrementStateOnNextTick)
    (Variables|Default|Set_IncrementStateOnNextTick false)
    (CallFunction|IncrementState true)))

(fn ConstructionScript)

(fn IncrementState
  (params (Skipped :type Boolean))
  (if (not (Utilities|HasWon))
    (CallFunction|ChangeState (Utilities|Enum|ByteToEnumE_GameOverlordState (+ (Variables|Default|GetState) 1)) Skipped)))

(fn ResetState
  (if (not (Utilities|HasWon))
    (CallFunction|ChangeState (Variables|Default|GetState) false)))

(fn ChangeState
  (params (NewState :type E_GameOverlordState%20Enum :default "NewEnumerator0") (Skipped :type Boolean))
  (bind __vrpawn (Variables|Default|Get_VRPawn))
  (Utilities|FlowControl|Sequence
    (:then_0
      ;[0.15 0.15 0.15 0.5] Debug Printing
      (CallFunction|DebugPrint true (Utilities|String|ToString(Text) (Utilities|Text|FormatText "Switching to state {state}" (Utilities|String|EnumtoString NewState)))))
    (:then_1
      ;[0.15 0.15 0.15 0.5] Unbind/delete old state objects
      (for _array_element (Variables|Default|GetCurrentChallenge)
        (if (Utilities|IsValid _array_element)
          (EventDispatchers|UnbindEventfromOnChallengeResolved _array_element (EventDispatchers|CreateEvent :!event Custom|OnVictory))
          (if (not (Utilities|WillWin NewState))
            (if Skipped
              (Default|CleanupChallenge _array_element))))))
    (:then_2
      ;[0.15 0.15 0.15 0.5] Close state-based menus
      (Utilities|IsValid __vrpawn
        (:Is%20Valid
          (bind _active (Default|IsMenuOpen __vrpawn true "NewEnumerator1"))
          (bind _active_2 (Default|IsMenuOpen __vrpawn true "NewEnumerator0"))
          (if (and _active (not _active_2))
            (Default|CloseMenu (Variables|Default|Get_VRPawn) false)))))
    (:then_3
      ;[0.15 0.15 0.15 0.5] Set State & Possibly Transition
      (bind _output_get (Variables|Default|SetState NewState))
      (switch Utilities|FlowControl|Switch|SwitchonE_GameOverlordState _output_get
        (:NewEnumerator0
          (Variables|Default|SetIsTransitioning false :!label _label)
          (CallFunction|InitState))
        (:NewEnumerator13
          (Variables|Default|SetIsTransitioning true :!label _label_2)
          (Default|Next (Variables|Default|Get_RailManager)))
        (:NewEnumerator10
          (goto _label_2))
        (:NewEnumerator1
          (goto _label))
        (:NewEnumerator11
          (goto _label_2))
        (:NewEnumerator14
          (goto _label_2))
        (:NewEnumerator3
          (goto _label_2))
        (:NewEnumerator8
          (goto _label))))))

(fn InitState
  (Utilities|Array|Clear (Variables|Default|GetCurrentChallenge))
  (Utilities|FlowControl|Sequence
    (:then_0
      (switch Utilities|FlowControl|Switch|SwitchonE_GameOverlordState (Variables|Default|GetState)
        (:NewEnumerator0
          ;[0.15 0.15 0.15 0.5] C-1: Spawn Main Title
          (Audio|SpawnSound2D "/Game/VRyu/Audio/Content/GameStart.GameStart" 1.0 1.0 0.2 0)
          (Utilities|FlowControl|Sequence
            (:then_0
              (Default|Disable (Variables|Default|GetSlicingLantern)))
            (:then_1
              (bind _returnvalue (Actor|GetActorOfClass "/Game/VRTemplate/Blueprints/VRPawn.VRPawn_C"))
              (Utilities|IsValid _returnvalue
                (:Is%20Valid
                  (Default|OpenMenu _returnvalue "NewEnumerator1" false))
                (:Is%20Not%20Valid
                  (Development|PrintString "ERROR: no player pawn detected, cannot begin challenge sequence" true true "(R=1.000000,G=0.000000,B=0.000000,A=1.000000)" 4.0)
                  (Variables|Default|Set_IncrementStateOnNextTick true))))))
        (:NewEnumerator13
          ;[0.15 0.15 0.15 0.5] C0: Select Weapon
          (Variables|Default|SetCurrentChallenge (Variables|Default|GetC0:%20Select%20Weapon)))
        (:NewEnumerator10
          ;[0.15 0.15 0.15 0.5] C1: Bamboo Tameshigiri
          (Variables|Default|SetCurrentChallenge (Utilities|Array|MakeArray (Variables|Default|GetC1:%20Bamboo)))
          (Default|Enable (Variables|Default|GetSlicingLantern)))
        (:NewEnumerator1
          ;[0.15 0.15 0.15 0.5] C2: Watermelon Launcher
          (Variables|Default|SetCurrentChallenge (Utilities|Array|MakeArray (Variables|Default|GetC2:%20Launcher))))
        (:NewEnumerator11
          ;[0.15 0.15 0.15 0.5] C3: Enemy
          (Variables|Default|SetCurrentChallenge (Utilities|Array|MakeArray (Variables|Default|GetC3:%20Enemy)))
          (Default|Disable (Variables|Default|GetSlicingLantern)))
        (:NewEnumerator14
          ;[0.15 0.15 0.15 0.5] C3.5: Enemies (Part 2)
          (Variables|Default|SetCurrentChallenge (Utilities|Array|MakeArray (Variables|Default|GetC3-5:%20Enemies))))
        (:NewEnumerator3
          ;[0.15 0.15 0.15 0.5] C4: Teacup
          (Variables|Default|SetCurrentChallenge (Utilities|Array|MakeArray (Variables|Default|GetC4:%20Teacup)))
          (CallFunction|DropYourWeapons))
        (:NewEnumerator8
          ;[0.15 0.15 0.15 0.5] Show Credits/End Menu
          (bind _returnvalue_2 (Actor|GetActorOfClass "/Game/VRTemplate/Blueprints/VRPawn.VRPawn_C"))
          (Utilities|IsValid _returnvalue_2
            (:Is%20Valid
              (Default|OpenMenu _returnvalue_2 "NewEnumerator2" false))
            (:Is%20Not%20Valid
              (Development|PrintString "ERROR: no player pawn detected, cannot begin challenge sequence" true true "(R=1.000000,G=0.000000,B=0.000000,A=1.000000)" 4.0))))))
    (:then_1
      ;[0.15 0.15 0.15 0.5] Bind Completion Event
      (for _array_element (Variables|Default|GetCurrentChallenge)
        (if (Utilities|IsValid _array_element)
          (EventDispatchers|BindEventtoOnChallengeResolved _array_element (EventDispatchers|CreateEvent :!event Custom|OnVictory))
          (Default|StartChallenge _array_element))))))

(fn RestartChallenge
  (for _array_element (Variables|Default|GetCurrentChallenge)
    (Utilities|IsValid _array_element
      (:Is%20Valid
        (Default|ResetChallenge _array_element)
        (Default|StartChallenge _array_element)))))

(fn CanRestartChallenge
  (if (Variables|Default|GetIsTransitioning)
    (return false)
    (elif (Utilities|Array|IsEmpty (Variables|Default|GetCurrentChallenge))
      (return false)
      (else
        (Utilities|FlowControl|Sequence
          (:then_0
            ;[0.15 0.15 0.15 0.5] Deny if any challenge can't be reset
            (for _array_element (Variables|Default|GetCurrentChallenge)
              (if (and (Utilities|IsValid _array_element) (not (Default|CanbeReset _array_element)))
                (return false))))
          (:then_1
            (return true)))))))

(fn DropYourWeapons
  (bind _outactors (Actor|GetAllActorsOfClass "/Game/VRyu/Blueprints/BP_Sword.BP_Sword_C"))
  (for _array_element _outactors
    (if (Variables|/Game/VRTemplate/Blueprints/GrabComponent.GrabComponent_C|GetbIsHeld (Variables|/Game/VRyu/Blueprints/BP_Sword.BP_Sword_C|GetGrabHandle _array_element))
      (Default|TryRelease (Variables|/Game/VRyu/Blueprints/BP_Sword.BP_Sword_C|GetGrabHandle _array_element))
      (Variables|/Game/VRTemplate/Blueprints/GrabComponent.GrabComponent_C|SetGrabResponse (Variables|/Game/VRyu/Blueprints/BP_Sword.BP_Sword_C|GetGrabHandle _array_element) "NewEnumerator2")
      (Rendering|SetVisibility (Variables|/Script/Engine.Actor|GetRootComponent _array_element) false true))))

(fn DebugPrint
  (params (bEnabled :type Boolean) (str :type String))
  (if (and bEnabled (Variables|Default|GetbDebugMode))
    (Development|PrintString (Utilities|String|ToString(Text) (Utilities|Text|FormatText "[BP_RoomOverlord]: {String}" str)) true true "(R=0.000000,G=0.043654,B=1.000000,A=1.000000)")))

(fn DebugInit)