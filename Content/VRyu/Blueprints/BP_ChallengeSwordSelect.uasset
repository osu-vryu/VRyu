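; VR challenge where the player picks one of several swords, each in a sheath with decals and configurable meshes and trail/particle colours.
; The child BP_Sword stays ungrabbable until StartChallenge restores its grab response.
; First grab attaches the sheath to the katana and disables all other selection swords.
; After a delay it plays audio, destroys sheath and decals, then signals OnChallengeBeat; the challenge cannot be reset.
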(event Custom|ExecuteDespawnSequence
  ;[0.15 0.15 0.15 0.5] When sword grabbed, run this custom event. This event is called from BP_Sword.
  (bind _childsword (Utilities|GetChildSword)
    (:Succeeded
      ;[0.15 0.15 0.15 0.5 16] After Cast, we now have reference to BP_Sword, so, grab Katana ref and do Attatch Comp to Comp, to bind the Local sheathe, to the Katana.
      (Transformation|AttachComponentToComponent (Variables|Default|GetSheathContainer) (Variables|/Game/VRyu/Blueprints/BP_Sword.BP_Sword_C|GetKatana _childsword) "None" "KeepRelative" "KeepRelative" "KeepRelative" true)
      (Utilities|FlowControl|Sequence
        (:then_0
          ;[0.15 0.15 0.15 0.5] Make all other swords ungrabbable, to prevent grabbing multiple (however cool that would be)
          (bind _outactors (Actor|GetAllActorsOfClass "BP_ChallengeSwordSelect_C"))
          (for _array_element _outactors
            (if (!= _array_element self)
              (CallFunction|DisableSword _array_element))))
        (:then_1
          ;[0.15 0.15 0.15 0.5 16] Remove Meshes after 5s delay. TODO: dissolve material + user keystroke to begin rather than delay
          (Utilities|FlowControl|Delay 4.0)
          (Audio|Components|Audio|Play (Variables|Default|GetAudioPlayer) 0.0)
          (Utilities|FlowControl|Delay 0.3)
          (Components|DestroyComponent (Variables|Default|GetSheathContainer))
          (Components|DestroyComponent (Variables|Default|Getdecals))
          ;[0.06125 0.06125 0.06125 1 16] indicates back to overlord that this is done.
          (Default|CallOnChallengeBeat))))))

(event EventBeginPlay
  (|CallParentFunction)
  (bind _childsword (Utilities|GetChildSword)
    (:Succeeded
      (Utilities|FlowControl|Sequence
        (:then_0
          (Variables|Default|Set_NormalGrabResponse (Variables|/Game/VRTemplate/Blueprints/GrabComponent.GrabComponent_C|GetGrabResponse (Variables|/Game/VRyu/Blueprints/BP_Sword.BP_Sword_C|GetGrabHandle _childsword)))
          (Variables|/Game/VRTemplate/Blueprints/GrabComponent.GrabComponent_C|SetGrabResponse (Variables|/Game/VRyu/Blueprints/BP_Sword.BP_Sword_C|GetGrabHandle _childsword) "NewEnumerator2"))
        (:then_1
          ;[0.15 0.15 0.15 0.5] When sword grabbed, run this custom event. This event is called from BP_Sword.
          (EventDispatchers|BindEventtoOnSwordFirstGrabbed _childsword (delegate Custom|ExecuteDespawnSequence)))))))

(event Collision|EventActorBeginOverlap
  (params (OtherActor :type Actor%20Object%20Reference)))

(event EventTick
  (params (DeltaSeconds :type Float%20%28single-precision%29)))

(fn ConstructionScript
  (bind _sheathoverride (Variables|Default|GetSheathOverride))
  (bind _decaloverride (Variables|Default|GetDecalOverride))
  (Utilities|FlowControl|Sequence
    (:then_0
      ;[0.15 0.15 0.15 0.5] On construction, check if SheathOverride was set (is valid), if it is, set it to the sheathe mesh.
      (Utilities|IsValid _sheathoverride
        (:Is%20Valid
          (Components|StaticMesh|SetStaticMesh (Variables|Default|GetSheathContainer) _sheathoverride))))
    (:then_1
      ;[0.15 0.15 0.15 0.5] same process, but for decals
      (Utilities|IsValid _decaloverride
        (:Is%20Valid
          (Components|StaticMesh|SetStaticMesh (Variables|Default|Getdecals) _decaloverride))))
    (:then_2
      ;[0.15 0.15 0.15 0.5] Assign blade's color attribute(s)
      (bind _childsword (Utilities|GetChildSword)
        (:Succeeded
          (Variables|/Game/VRyu/Blueprints/BP_Sword.BP_Sword_C|SetTrailColor _childsword (Variables|Default|GetTrailColor))
          (Variables|/Game/VRyu/Blueprints/BP_Sword.BP_Sword_C|SetParticlesColor _childsword (Variables|Default|GetParticlesColor)))))))

(fn CanbeReset
  (return false))

(fn StartChallenge
  (|CallParentFunction)
  (bind _childsword (Utilities|GetChildSword)
    (:Succeeded
      (Variables|/Game/VRTemplate/Blueprints/GrabComponent.GrabComponent_C|SetGrabResponse (Variables|/Game/VRyu/Blueprints/BP_Sword.BP_Sword_C|GetGrabHandle _childsword) (Variables|Default|Get_NormalGrabResponse)))))

(fn ResetChallenge
  (|CallParentFunction))

(fn CleanupChallenge
  (|CallParentFunction)
  (CallFunction|DisableSword))

(fn DisableSword
  (bind _childsword (Utilities|GetChildSword)
    (:Succeeded
      (Variables|/Game/VRTemplate/Blueprints/GrabComponent.GrabComponent_C|SetGrabResponse (Variables|/Game/VRyu/Blueprints/BP_Sword.BP_Sword_C|GetGrabHandle _childsword) "NewEnumerator2"))))