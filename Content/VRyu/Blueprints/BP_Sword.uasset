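; VR grabbable sword that slices BPI_Sliceable objects while held or flagged always active, with its mesh overridable by parent BP_Select_Weapon.
; Tick attempts slices on overlapped components and on hits from substepped sweeps of the absolute-transform blade hitbox, faking continuous collision.
; Strikes use hand velocity, or a frame-buffer average as fallback, projected onto blade forward.
; Results drive haptics and a sliced event; an active blade disables regular collision.
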(event Custom|BladeHitboxBeginOverlap
  (params (OverlappedComponent :type Primitive%20Component%20Object%20Reference) (OtherActor :type Actor%20Object%20Reference) (OtherComp :type Primitive%20Component%20Object%20Reference) (OtherBodyIndex :type Integer) (bFromSweep :type Boolean) (SweepResult :type Hit%20Result%20Structure%20%28by%20ref%29))
  (bind _overlapedsliceables (Variables|Default|GetOverlapedSliceables))
  (bind (_value _returnvalue) (Utilities|Map|Find _overlapedsliceables OtherActor))
  ;[0.15 0.15 0.15 0.5] Track overlapping sliceables
  (bind _isactive (CallFunction|IsBladeActive))
  (if (and _isactive (== OverlappedComponent (Variables|Default|GetBlade%20Hitbox)))
    (Utilities|Casting|CastToBPI_Sliceable OtherActor)
    ;;[0.15 0.15 0.15 0.5] Add to map/set
    (if _returnvalue
      (Utilities|Array|AddUnique (Utilities|Struct|BreakS_BladeOverlapedComponents _value) OtherComp)
      (else
        (Utilities|Map|Add _overlapedsliceables OtherActor (Utilities|Struct|MakeS_BladeOverlapedComponents (Utilities|Array|MakeArray OtherComp)))))))

(event Custom|BladeHitboxEndOverlap
  (params (OverlappedComponent :type Primitive%20Component%20Object%20Reference) (OtherActor :type Actor%20Object%20Reference) (OtherComp :type Primitive%20Component%20Object%20Reference) (OtherBodyIndex :type Integer))
  (bind _overlapedsliceables (Variables|Default|GetOverlapedSliceables))
  (bind (_value _returnvalue) (Utilities|Map|Find _overlapedsliceables OtherActor))
  (bind _hitcomponents (Utilities|Struct|BreakS_BladeOverlapedComponents _value))
  ;[0.15 0.15 0.15 0.5] Track overlapping sliceables
  (if (== OverlappedComponent (Variables|Default|GetBlade%20Hitbox))
    ;;[0.15 0.15 0.15 0.5] Must be removed regardless of active state
    (Utilities|Casting|CastToBPI_Sliceable OtherActor)
    ;;[0.15 0.15 0.15 0.5] Remove from set/map
    (if _returnvalue
      (Utilities|Array|RemoveItem _hitcomponents OtherComp)
      (if (<= (Utilities|Array|Length _hitcomponents) 0)
        (Utilities|Map|Remove (Variables|Default|GetOverlapedSliceables) OtherActor)))))

(event Custom|OnGrabbed
  (Variables|Default|Set_FirstGrabMove true)
  ;[0.15 0.15 0.15 0.5 14] Call this event in BP_Select_Weapon
  (Default|CallOnSwordFirstGrabbed))

(event EventBeginPlay
  (bind _blade_hitbox (Variables|Default|GetBlade%20Hitbox))
  (Utilities|FlowControl|Sequence
    (:then_0
      ;[0.15 0.15 0.15 0.5] Initialize Vars
      (Variables|Default|Set_OriginalHoldingAngle (.Pitch (Math|Rotator|BreakRotator (Variables|/Script/Engine.SceneComponent|GetRelativeRotation (Variables|Default|GetGrabHandle)))))
      (Variables|Default|Set_FirstGrabMove true)
      (Variables|Default|Set_BladeLocalTransform (Transformation|GetRelativeTransform (Variables|Default|GetBlade%20Hitbox)))
      (Transformation|SetAbsolute (Variables|Default|GetBlade%20Hitbox) true true true)
      (Utilities|Map|Clear (Variables|Default|GetOverlapedSliceables)))
    (:then_1
      (Utilities|FlowControl|Sequence
        (:then_0
          (bind _asbp_vryu_game_instance (Utilities|Casting|CastToBP_VRyuGameInstance (Game|GetGameInstance)))
          (Default|UpdateBladeAngle _asbp_vryu_game_instance (Default|GetBladeAngle _asbp_vryu_game_instance)))
        (:then_1
          (bind _returnvalue (Actor|GetActorOfClass "/Game/VRTemplate/Blueprints/VRPawn.VRPawn_C"))
          (Utilities|IsValid _returnvalue
            (:Is%20Valid
              (Variables|Default|SetVRPawn _returnvalue))))))
    (:then_2
      (Collision|BindEventtoOnComponentBeginOverlap _blade_hitbox (delegate Custom|BladeHitboxBeginOverlap))
      (Collision|BindEventtoOnComponentEndOverlap _blade_hitbox (delegate Custom|BladeHitboxEndOverlap))
      (EventDispatchers|BindEventtoOnGrabbed (Variables|Default|GetGrabHandle) (delegate Custom|OnGrabbed)))))

(event EventTick
  (params (DeltaSeconds :type Float%20%28single-precision%29))
  (bind _blade_hitbox (Variables|Default|GetBlade%20Hitbox))
  (bind _collision_hitbox (Variables|Default|GetCollision%20Hitbox))
  (Utilities|FlowControl|Sequence
    (:then_0
      (CallFunction|PushBladeState DeltaSeconds))
    (:then_1
      (CallFunction|TickFakeContinuousCollision (not (Variables|Default|Get_FirstGrabMove)))
      (Variables|Default|Set_FirstGrabMove false))
    (:then_2
      ;[0.15 0.15 0.15 0.5] Slice overlapping meshes every tick
      (bind _isactive (CallFunction|IsBladeActive))
      (if _isactive
        (bind _keys (Utilities|Map|Keys (Variables|Default|GetOverlapedSliceables)))
        (for _index (range 0 (- (Utilities|Array|Length _keys) 1))
          (bind _asbpi_sliceable (Utilities|Casting|CastToBPI_Sliceable (Utilities|Array|Get(acopy) _keys (- (- (Utilities|Array|Length _keys) 1) _index)))
            (:then
              (if (and (Utilities|IsValidInterface _asbpi_sliceable) (.ReturnValue (Utilities|Map|Find (Variables|Default|GetOverlapedSliceables) (Utilities|Array|Get(acopy) _keys (- (- (Utilities|Array|Length _keys) 1) _index)))))
                (for _array_element (Utilities|Struct|BreakS_BladeOverlapedComponents (.Value (Utilities|Map|Find (Variables|Default|GetOverlapedSliceables) (Utilities|Array|Get(acopy) _keys (- (- (Utilities|Array|Length _keys) 1) _index)))))
                  (if (Utilities|IsValidInterface _asbpi_sliceable)
                    (CallFunction|AttemptSlice _asbpi_sliceable _array_element)))
                (else
                  (Utilities|Array|RemoveIndex _keys (- (- (Utilities|Array|Length _keys) 1) _index) :!label _label))))
            (:CastFailed
              (goto _label))))))
    (:then_3
      ;[0.15 0.15 0.15 0.5] Disable Regular Collision When Active
      (bind _isactive_2 (CallFunction|IsBladeActive))
      (if _isactive_2
        (Collision|SetCollisionEnabled _collision_hitbox "NoCollision")
        (Collision|SetCollisionEnabled _blade_hitbox "QueryAndPhysics")
        (else
          (Collision|SetCollisionEnabled _collision_hitbox "QueryAndPhysics")
          (Collision|SetCollisionEnabled _blade_hitbox "NoCollision"))))))

(fn ConstructionScript
  ;[0.15 0.15 0.15 0.5] Construction Script -> runs every time this BP is moved or changed in editor(?). This setup makes it so that Katana (the local instance of the mesh within this BP) is overriden with what mesh is SET in SwordMeshOverride (from BP_Select_Weapon).
  (bind _asbp_select_weapon (Utilities|Casting|CastToBP_Select_Weapon (Actor|GetParentActor)))
  (Utilities|IsValid (Variables|/Game/VRyu/Blueprints/BP_Select_Weapon.BP_Select_Weapon_C|GetSwordOverride _asbp_select_weapon)
    (:Is%20Valid
      (Components|StaticMesh|SetStaticMesh (Variables|Default|GetKatana) (Variables|/Game/VRyu/Blueprints/BP_Select_Weapon.BP_Select_Weapon_C|GetSwordOverride _asbp_select_weapon)))))

(fn IsBladeActive
  (if (Variables|Default|GetActiveWhenNotHeld)
    (return true)
    (else
      (return (Variables|/Game/VRTemplate/Blueprints/GrabComponent.GrabComponent_C|GetbIsHeld (Variables|Default|GetGrabHandle))))))

(fn PushBladeState
  (params (DeltaTime :type Float%20%28double-precision%29))
  (bind _bladestatebuffer (Variables|Default|GetBladeStateBuffer))
  (bind _returnvalue (Utilities|Array|Length _bladestatebuffer))
  (Utilities|Array|Insert (Variables|Default|GetBladeStateBuffer) (Utilities|Struct|MakeS_BladeFrameState (Transformation|GetWorldLocation (Variables|Default|GetEndTracker)) (Transformation|GetWorldRotation (Variables|Default|GetGrabHandle)) DeltaTime))
  (while (> _returnvalue (Variables|Default|GetBladeStateBufferSize))
    (Utilities|Array|RemoveIndex (Variables|Default|GetBladeStateBuffer) (- _returnvalue 1))))

(fn CalcAveVelocity
  (params (MaxTime :type Float%20%28double-precision%29))
  (bind _bladestatebuffer (Variables|Default|GetBladeStateBuffer))
  (bind _bladestatebuffer_2 (Variables|Default|GetBladeStateBuffer))
  (bind _returnvalue (Utilities|Array|Length _bladestatebuffer))
  (if (< _returnvalue 2)
    (return "0, 0, 0")
    (else
      (bind _index (Utilities|FlowControl|ForLoopwithBreak 0 (- _returnvalue 2) :!label _label)
        (:LoopBody
          (if (>= (+ (.DeltaTime (Utilities|Struct|BreakS_BladeFrameState (Utilities|Array|Get(acopy) _bladestatebuffer_2 _index))) (LocalVariables|GetTimeSum)) MaxTime)
            (goto _label Break)
            (else
              (LocalVariables|SetTimeSum (+ (.DeltaTime (Utilities|Struct|BreakS_BladeFrameState (Utilities|Array|Get(acopy) _bladestatebuffer_2 _index))) (LocalVariables|GetTimeSum)))
              (LocalVariables|SetVelSum (+ (- (.EndPosition (Utilities|Struct|BreakS_BladeFrameState (Utilities|Array|Get(acopy) _bladestatebuffer_2 _index))) (.EndPosition (Utilities|Struct|BreakS_BladeFrameState (Utilities|Array|Get(acopy) _bladestatebuffer_2 (+ _index 1))))) (LocalVariables|GetVelSum))))))
        (:Completed
          (if (<= (LocalVariables|GetTimeSum) 0.0)
            (return "0, 0, 0")
            (else
              (return (/ (LocalVariables|GetVelSum) (- (Utilities|Array|Length (Variables|Default|GetBladeStateBuffer)) 1))))))))))

(fn AttemptSlice
  (params (Sliceable :type BPI%20Sliceable%20Interface) (HitComponent :type Primitive%20Component%20Object%20Reference))
  (bind _grabhandle (Variables|Default|GetGrabHandle))
  (bind _blade_hitbox (Variables|Default|GetBlade%20Hitbox))
  (bind _vrpawn (Variables|Default|GetVRPawn))
  (bind _grabhandle_2 (Variables|Default|GetGrabHandle))
  (bind _returnvalue (Default|GetHeldbyHand _grabhandle_2))
  (bind _returnvalue_2 (Math|Vector|GetForwardVector _blade_hitbox))
  (bind _isheldby (Variables|/Game/VRTemplate/Blueprints/GrabComponent.GrabComponent_C|GetisHeldBy _grabhandle))
  (bind (_outlinearvelocity _returnvalue_3) (Class|MotionControllerComponent|GetLinearVelocity _isheldby))
  (CallFunction|DebugPrint false "Starting slice attempt")
  ;[0.15 0.15 0.15 0.5] Get blade velocity
  (if (Variables|/Game/VRTemplate/Blueprints/GrabComponent.GrabComponent_C|GetbIsHeld (Variables|Default|GetGrabHandle))
    (Utilities|IsValid _isheldby
      (:Is%20Valid
        (if _returnvalue_3
          (LocalVariables|SetVelocity _outlinearvelocity)
          (else
            (bind _velocity (CallFunction|CalcAveVelocity 1.0 :!label _label))
            (LocalVariables|SetVelocity _velocity))))
      (:Is%20Not%20Valid
        (goto _label)))
    (else
      (goto _label)))
  (bind _sliceresult (Default|TrySlice Sliceable (Transformation|GetWorldLocation (Variables|Default|GetGrabHandle)) (Math|Vector|GetUpVector _blade_hitbox) (* (Math|Float|Max(Float) (Math|Vector|DotProduct (LocalVariables|GetVelocity) _returnvalue_2) 0.0) _returnvalue_2) HitComponent))
  (Utilities|FlowControl|Sequence
    (:then_0
      (switch Utilities|FlowControl|Switch|SwitchonE_SliceResult _sliceresult
        (:NewEnumerator0
          (Default|CallSlicedObject))))
    (:then_1
      ;[0.15 0.15 0.15 0.5] Haptic Response
      (Utilities|IsValid _vrpawn
        (:Is%20Valid
          (switch Utilities|FlowControl|Switch|SwitchonE_SliceResult _sliceresult
            (:NewEnumerator0
              (Default|PlayHaptic _vrpawn "/Game/VRTemplate/Haptics/H_SliceSuccess.H_SliceSuccess" _returnvalue false))
            (:NewEnumerator1
              (if (>= (- (Utilities|Time|GetGameTimeinSeconds) (Variables|Default|Get_TimeLastSentHapticResponse)) (Variables|Default|Get_MinTimeBetweenAlmostHaptics))
                (Default|PlayHaptic _vrpawn "/Game/VRTemplate/Haptics/H_SliceAlmost.H_SliceAlmost" _returnvalue false))))
          (Variables|Default|Set_TimeLastSentHapticResponse (Utilities|Time|GetGameTimeinSeconds)))))
    (:then_2
      (return _sliceresult))))

(fn DebugPrint
  (params (bEnabled :type Boolean) (str :type String))
  (if (and bEnabled (Variables|Default|GetbDebugMode))
    (Development|PrintString (Utilities|String|ToString(Text) (Utilities|Text|FormatText "[BP_Sword]: {String}" str)))))

(fn SetHoldingAngle
  (params (NewAngle :type Float%20%28double-precision%29))
  (bind _grabhandle (Variables|Default|GetGrabHandle))
  (bind _relativerotation (Variables|/Script/Engine.SceneComponent|GetRelativeRotation _grabhandle))
  (bind (_roll _pitch _yaw) (Math|Rotator|BreakRotator _relativerotation))
  (bind _output_get (Variables|Default|SetHoldingAngle NewAngle))
  (Transformation|SetRelativeRotation _grabhandle (Math|Rotator|CombineRotators (Math|Rotator|MakeRotator _roll (Variables|Default|Get_OriginalHoldingAngle) _yaw) (Math|Rotator|MakeRotator 0.0 _output_get 0.0)) false true))

(fn TickFakeContinuousCollision
  (params (DoSweep :type Boolean))
  (bind _sweepsubsteps (Variables|Default|GetSweepSubsteps))
  (LocalVariables|SetStartTransform (Transformation|GetWorldTransform (Variables|Default|GetBlade%20Hitbox)))
  (LocalVariables|SetEndTransform (Math|Transform|ComposeTransforms (Variables|Default|Get_BladeLocalTransform) (Transformation|GetActorTransform)))
  (Utilities|FlowControl|Sequence
    (:then_0
      (if DoSweep
        (Utilities|FlowControl|Sequence
          (:then_0
            (for _index (range 1 _sweepsubsteps)
              (bind _sweephitresult (Transformation|SetWorldLocationAndRotation (Variables|Default|GetBlade%20Hitbox) (.Location (Math|Transform|BreakTransform (Math|Transform|Lerp(Transform) (LocalVariables|GetStartTransform) (LocalVariables|GetEndTransform) (/ _index (Math|Conversions|ToFloat(Integer) _sweepsubsteps))))) (.Rotation (Math|Transform|BreakTransform (Math|Transform|Lerp(Transform) (LocalVariables|GetStartTransform) (LocalVariables|GetEndTransform) (/ _index (Math|Conversions|ToFloat(Integer) _sweepsubsteps))))) true true))
              (if (or (.bBlockingHit (Collision|BreakHitResult _sweephitresult)) (.bInitialOverlap (Collision|BreakHitResult _sweephitresult)))
                (bind _asbpi_sliceable (Utilities|Casting|CastToBPI_Sliceable (.HitActor (Collision|BreakHitResult _sweephitresult))))
                (Utilities|Array|AddUnique (LocalVariables|GetSweptComponents) (Utilities|Struct|MakeS_BladeSweptComponents _asbpi_sliceable (.HitComponent (Collision|BreakHitResult _sweephitresult)))))))
          (:then_1
            (for _array_element (LocalVariables|GetSweptComponents)
              (CallFunction|AttemptSlice (.Sliceable (Utilities|Struct|BreakS_BladeSweptComponents _array_element)) (.HitComponent (Utilities|Struct|BreakS_BladeSweptComponents _array_element))))))))
    (:then_1
      (Transformation|SetWorldLocationAndRotation (Variables|Default|GetBlade%20Hitbox) (.Location (Math|Transform|BreakTransform (LocalVariables|GetEndTransform))) (.Rotation (Math|Transform|BreakTransform (LocalVariables|GetEndTransform))) false true))))