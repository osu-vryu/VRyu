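; Melee enemy that chases the player, attacks in range and can block or die from sword slices.
; A looping PollChase timer moves it by AI toward the player and sets state flags, pausing after hits.
; TrySlice treats hits on its sword hitbox during attacks as blocks that stagger it backward.
; Body hits kill it, turning partial physical animation into ragdoll, signaling defeat and slowing global time.
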(event Custom|PollChase
  (bind _returnvalue (Game|Player|GetPlayerPawn 0))
  (bind _self self)
  (if (Variables|Default|GetbIsHit)
    (Utilities|FlowControl|Delay 1.2)
    (Variables|Default|SetbIsHit false)
    (elif (<= (Transformation|GetDistanceTo _self _returnvalue) (Variables|Default|GetAttackRange))
      (AI|Navigation|StopMovement (AI|GetAIController self))
      (Variables|Default|SetbIsAttacking true)
      (Variables|Default|SetbIsMoving false)
      (else
        (AI|AIMoveTo _self "0, 0, 0" _returnvalue 5.0 false
          (:then
            (Variables|Default|SetbIsMoving true)
            (Variables|Default|SetbIsAttacking false)))))))

(event Custom|ChasePlayer
  (Utilities|Time|SetTimerbyFunctionName 0 "PollChase" 0.4 true true))

(event EventBeginPlay
  (Variables|Default|SetbIsAlive true)
  (Variables|Default|SetbIsHit false)
  (Variables|Default|SetbIsMoving false)
  (Variables|Default|SetbIsAttacking false)
  (Class|PhysicalAnimationComponent|SetSkeletalMeshComponent (Variables|Default|GetPhysicalAnimation) (Variables|Character|GetMesh))
  (Class|PhysicalAnimationComponent|ApplyPhysicalAnimationProfileBelow (Variables|Default|GetPhysicalAnimation) "Hips" "None" true false))

(fn ConstructionScript)

(fn TrySlice
  (params (SlicePos :type Vector :default "0, 0, 0") (SliceNormal :type Vector :default "0, 0, 0") (StrikeVel :type Vector :default "0, 0, 0") (HitComponent :type Primitive%20Component%20Object%20Reference))
  (bind _returnvalue (Utilities|String|StringToName "Hips"))
  (bind _mesh (Variables|Character|GetMesh))
  (bind _swordhitbox (Variables|Default|GetSwordHitbox))
  (if (Variables|Default|GetbIsAlive)
    (if (Math|Boolean|ANDBoolean (not (Variables|Default|GetbIsHit)) (== HitComponent _swordhitbox) (Variables|/Script/Engine.PrimitiveComponent|GetbGenerateOverlapEvents _swordhitbox) (Variables|Default|GetbIsAttacking))
      ;[0.15 0.15 0.15 0.5] Enemy Block
      (Audio|PlaySoundatLocation "/Game/VRyu/Audio/Content/SliceMetal.SliceMetal" (Transformation|GetWorldLocation (Variables|Default|GetSwordHitbox)) "0, 0, 0" 1.0 (Math|Random|RandomFloatinRange 0.9 1.1) 0.0 0 0 0 0)
      (Variables|Default|SetbIsHit true)
      (Variables|Default|SetbIsMoving false)
      (Variables|Default|SetbIsAttacking false)
      (Character|LaunchCharacter (* (Math|Vector|Normalize (- (Transformation|GetActorLocation) (Transformation|GetActorLocation (Game|Player|GetPlayerPawn 0)))) (Variables|Default|GetStagger)) false true)
      (return "NewEnumerator0")
      (elif (!= _swordhitbox HitComponent)
        (Variables|Default|SetbIsAlive false)
        ;[0.15 0.15 0.15 0.5] Enemy Death
        (Audio|PlaySoundatLocation "/Game/VRyu/Audio/Content/woodthunk.woodthunk" (Transformation|GetWorldLocation (Variables|Default|GetSwordHitbox)) "0, 0, 0" 1.0 (Math|Random|RandomFloatinRange 0.9 1.1) 0.0 0 0 0 0)
        (Utilities|FlowControl|Sequence
          (:then_0
            (Utilities|FlowControl|Sequence
              (:then_0
                (Variables|Default|SetbIsMoving false)
                (Variables|Default|SetbIsAttacking false))
              (:then_1
                (Class|SkeletalMeshComponent|SetAllBodiesSimulatePhysics (Variables|Character|GetMesh) true)
                (Class|SkeletalMeshComponent|SetAllBodiesBelowPhysicsBlendWeight _mesh _returnvalue 1.0 false true)
                (Class|SkeletalMeshComponent|SetEnableGravityonAllBodiesBelow _mesh true _returnvalue true)
                (Audio|Components|Audio|Stop (Variables|Character|GetMesh)))
              (:then_2
                (Default|CallOnEnemyDefeated self))
              (:then_3
                (Utilities|Time|SetGlobalTimeDilation 0.7))))
          (:then_1
            (return "NewEnumerator0"))
          (:then_2
            (Development|PrintString "IS PLAYER" true true "(R=1.000000,G=0.000000,B=0.788692,A=1.000000)")))
        (else
          (return "NewEnumerator2"))))
    (else
      (return "NewEnumerator2"))))