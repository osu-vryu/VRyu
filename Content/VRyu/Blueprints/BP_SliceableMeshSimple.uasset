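; BP_SliceableMeshSimple is an actor built around a single StaticMesh component, named as a simple sliceable mesh.
; On BeginPlay it applies MeshOverride to that component when one is set, then calls the parent BeginPlay.
; GetStaticMesh exposes the component, and the file itself contains no slicing logic.
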(event EventBeginPlay
  (bind _meshoverride (Variables|Default|GetMeshOverride))
  (Utilities|IsValid _meshoverride
    (:Is%20Valid
      (Components|StaticMesh|SetStaticMesh (Variables|Default|GetStaticMesh) _meshoverride))
    (:Is%20Not%20Valid
      _))
  (|CallParentFunction))

(event Collision|EventActorBeginOverlap
  (params (OtherActor :type Actor%20Object%20Reference))
  (|CallParentFunction OtherActor) ; This node is disabled and will not be called.\nDrag off pins to build functionality.
)

(event EventTick
  (params (DeltaSeconds :type Float%20%28single-precision%29))
  (|CallParentFunction DeltaSeconds) ; This node is disabled and will not be called.\nDrag off pins to build functionality.
)

(fn ConstructionScript
  (|CallParentFunction))

(fn GetStaticMesh
  (return (Variables|Default|GetStaticMesh)))