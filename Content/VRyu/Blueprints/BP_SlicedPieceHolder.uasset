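; BP_SlicedPieceHolder is an actor that holds procedural mesh pieces cut from a sliceable object.
; It forwards overlap, hit and slice requests to its ParentSliceable, printing an error if a slice arrives with no valid parent.
; DestroyChild removes a piece component and destroys the actor once no procedural mesh components remain.
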(event EventBeginPlay)

(event EventTick
  (params (DeltaSeconds :type Float%20%28single-precision%29)))

(event Collision|EventHit
  (params (MyComp :type Primitive%20Component%20Object%20Reference) (Other :type Actor%20Object%20Reference) (OtherComp :type Primitive%20Component%20Object%20Reference) (bSelfMoved :type Boolean) (HitLocation :type Vector :default "0, 0, 0") (HitNormal :type Vector :default "0, 0, 0") (NormalImpulse :type Vector :default "0, 0, 0") (Hit :type Hit%20Result%20Structure%20%28by%20ref%29))
  (bind _parentsliceable (Variables|Default|GetParentSliceable))
  (|CallParentFunction MyComp Other OtherComp bSelfMoved HitLocation HitNormal NormalImpulse Hit)
  (Utilities|IsValid _parentsliceable
    (:Is%20Valid
      (Default|CallOnPieceHit _parentsliceable MyComp Other OtherComp bSelfMoved HitLocation HitNormal NormalImpulse Hit))))

(event Collision|EventActorBeginOverlap
  (params (OtherActor :type Actor%20Object%20Reference))
  (bind _parentsliceable (Variables|Default|GetParentSliceable))
  (|CallParentFunction OtherActor)
  (Utilities|IsValid _parentsliceable
    (:Is%20Valid
      (Default|CallOnPieceBeginOverlap _parentsliceable OtherActor))))

(event Collision|EventActorEndOverlap
  (params (OtherActor :type Actor%20Object%20Reference))
  (bind _parentsliceable (Variables|Default|GetParentSliceable))
  (|CallParentFunction OtherActor)
  (Utilities|IsValid _parentsliceable
    (:Is%20Valid
      (Default|CallOnPieceEndOverlap _parentsliceable OtherActor))))

(fn ConstructionScript)

(fn IsEmpty
  (return (not (Utilities|IsValid (Actor|GetComponentbyClass self "/Script/ProceduralMeshComponent.ProceduralMeshComponent")))))

(fn DestroyChild
  (params (Component :type Mesh%20Component%20Object%20Reference))
  (Components|DestroyComponent Component)
  (if (CallFunction|IsEmpty)
    (Actor|DestroyActor)))

(fn TrySlice
  (params (SlicePos :type Vector :default "0, 0, 0") (SliceNormal :type Vector :default "0, 0, 0") (StrikeVel :type Vector :default "0, 0, 0") (HitComponent :type Primitive%20Component%20Object%20Reference))
  (Utilities|IsValid (Variables|Default|GetParentSliceable)
    (:Is%20Valid
      (bind _sliceresult (Default|TrySlice (Variables|Default|GetParentSliceable) SlicePos SliceNormal StrikeVel HitComponent))
      (return _sliceresult))
    (:Is%20Not%20Valid
      (Development|PrintString "ERROR: no sliceable parentent to piece holder!" true true "(R=1.000000,G=0.000000,B=0.000000,A=1.000000)")
      (return "NewEnumerator2"))))