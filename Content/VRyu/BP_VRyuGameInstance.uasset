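; Game instance for the VRyu VR game that owns persistent player settings, background audio and event-keyed sound playback.
; Getters and updaters lazily load a BP_VRyuSaveGame, and each update saves it to the slot immediately.
; Blade angle, volume, resolution and height changes are also pushed to swords, the master sound mix, resolution scale and VR pawn.
; Init starts background audio that persists across level transitions.
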(event EventInit
  (Utilities|FlowControl|Delay 0.2)
  (bind _returnvalue (Audio|SpawnSound2D "/Game/VRyu/Audio/Content/Background.Background" 1.0 1.0 0.0 0 true false))
  (Variables|Default|SetAmbientAudioComponent _returnvalue))

(fn UpdateBladeAngle
  (params (NewAngle :type Float%20%28double-precision%29))
  (CallFunction|EnsureSettingsLoaded)
  (Variables|/Game/VRyu/BP_VRyuSaveGame.BP_VRyuSaveGame_C|SetBladeAngle (Variables|Default|GetSettings) NewAngle)
  (CallFunction|SaveSettings)
  (bind _outactors (Actor|GetAllActorsOfClass "/Game/VRyu/Blueprints/BP_Sword.BP_Sword_C"))
  (for _array_element _outactors
    (Default|SetHoldingAngle _array_element (Variables|/Game/VRyu/BP_VRyuSaveGame.BP_VRyuSaveGame_C|GetBladeAngle (Variables|Default|GetSettings)))
    (Default|RefreshGrabbedRotation (Variables|/Game/VRyu/Blueprints/BP_Sword.BP_Sword_C|GetGrabHandle _array_element))))

(fn UpdateVolume
  (params (NewVolume :type Float%20%28double-precision%29))
  (CallFunction|EnsureSettingsLoaded)
  (bind _output_get (Variables|/Game/VRyu/BP_VRyuSaveGame.BP_VRyuSaveGame_C|SetVolume (Variables|Default|GetSettings) (Math|Float|Max(Float) (Math|Float|Min(Float) NewVolume 1.0) 0.0)))
  (CallFunction|SaveSettings)
  (Class|GameplayStatics|ClearSoundMixModifiers)
  (Audio|SetSoundMixClassOverride "/Game/VRyu/Audio/SCM_MasterMix.SCM_MasterMix" "/Game/VRyu/Audio/SC_Master.SC_Master" _output_get 1.0 0.1 true)
  (Audio|PushSoundMixModifier "/Game/VRyu/Audio/SCM_MasterMix.SCM_MasterMix"))

(fn UpdateResolution
  (params (NewValue :type Float%20%28double-precision%29))
  (CallFunction|EnsureSettingsLoaded)
  (bind _output_get (Variables|/Game/VRyu/BP_VRyuSaveGame.BP_VRyuSaveGame_C|SetResolution (Variables|Default|GetSettings) NewValue))
  (CallFunction|SaveSettings)
  (bind _returnvalue (Settings|GetGameUserSettings))
  (Class|GameUserSettings|SetResolutionScaleNormalized _returnvalue _output_get)
  (Class|GameUserSettings|ApplyResolutionSettings _returnvalue true))

(fn UpdateHapticsMultiplier
  (params (NewMultiplier :type Float%20%28double-precision%29))
  (CallFunction|EnsureSettingsLoaded)
  (Variables|/Game/VRyu/BP_VRyuSaveGame.BP_VRyuSaveGame_C|SetHapticsMultiplier (Variables|Default|GetSettings) (Math|Float|Max(Float) (Math|Float|Min(Float) NewMultiplier 1.0) 0.0))
  (CallFunction|SaveSettings))

(fn UpdateMotionVignette
  (params (NewValue :type Boolean))
  (CallFunction|EnsureSettingsLoaded)
  (Variables|/Game/VRyu/BP_VRyuSaveGame.BP_VRyuSaveGame_C|SetMotionVignette (Variables|Default|GetSettings) NewValue)
  (CallFunction|SaveSettings))

(fn UpdateHeightOffset
  (params (NewHeightOffset :type Float%20%28double-precision%29))
  (CallFunction|EnsureSettingsLoaded)
  (Variables|/Game/VRyu/BP_VRyuSaveGame.BP_VRyuSaveGame_C|SetHeightOffset (Variables|Default|GetSettings) NewHeightOffset)
  (Utilities|FlowControl|Sequence
    (:then_0
      (CallFunction|SaveSettings))
    (:then_1
      (bind _returnvalue (Actor|GetActorOfClass "/Game/VRTemplate/Blueprints/VRPawn.VRPawn_C"))
      (Default|UpdateHeightOffset _returnvalue (Variables|/Game/VRyu/BP_VRyuSaveGame.BP_VRyuSaveGame_C|GetHeightOffset (Variables|Default|GetSettings))))))

(fn GetBladeAngle
  (CallFunction|EnsureSettingsLoaded)
  (return (Variables|/Game/VRyu/BP_VRyuSaveGame.BP_VRyuSaveGame_C|GetBladeAngle (Variables|Default|GetSettings))))

(fn GetVolume
  (CallFunction|EnsureSettingsLoaded)
  (return (Variables|/Game/VRyu/BP_VRyuSaveGame.BP_VRyuSaveGame_C|GetVolume (Variables|Default|GetSettings))))

(fn GetResolution
  (CallFunction|EnsureSettingsLoaded)
  (return (Variables|/Game/VRyu/BP_VRyuSaveGame.BP_VRyuSaveGame_C|GetResolution (Variables|Default|GetSettings))))

(fn GetHapticsMultiplier
  (CallFunction|EnsureSettingsLoaded)
  (return (Variables|/Game/VRyu/BP_VRyuSaveGame.BP_VRyuSaveGame_C|GetHapticsMultiplier (Variables|Default|GetSettings))))

(fn GetMotionVignette
  (CallFunction|EnsureSettingsLoaded)
  (return (Variables|/Game/VRyu/BP_VRyuSaveGame.BP_VRyuSaveGame_C|GetMotionVignette (Variables|Default|GetSettings))))

(fn GetHeightOffset
  (CallFunction|EnsureSettingsLoaded)
  (return (Variables|/Game/VRyu/BP_VRyuSaveGame.BP_VRyuSaveGame_C|GetHeightOffset (Variables|Default|GetSettings))))

(fn SaveSettings
  (CallFunction|EnsureSettingsLoaded)
  (bind _returnvalue (SaveGame|SaveGametoSlot (Variables|Default|GetSettings) (Variables|Default|GetSaveSlotName)))
  (if (not _returnvalue)
    (Development|PrintString "ERROR: save game failed to save!" true true "(R=1.000000,G=0.000000,B=0.000000,A=1.000000)")))

(fn EnsureSettingsLoaded
  (bind _saveslotname (Variables|Default|GetSaveSlotName))
  (if (or (not (Variables|Default|GetSettingsLoaded)) (not (Utilities|IsValid (Variables|Default|GetSettings))))
    (Utilities|FlowControl|Sequence
      (:then_0
        (bind _returnvalue (SaveGame|DoesSaveGameExist _saveslotname))
        (if _returnvalue
          (bind _returnvalue_2 (SaveGame|LoadGamefromSlot _saveslotname))
          (bind _asbp_vryu_save_game (Utilities|Casting|CastToBP_VRyuSaveGame _returnvalue_2)
            (:then
              (Variables|Default|SetSettings _asbp_vryu_save_game))
            (:CastFailed
              (Development|PrintString "ERROR: save game of wrong type; creating new one" true true "(R=1.000000,G=0.000000,B=0.000000,A=1.000000)")))
          (else
            (bind _returnvalue_3 (SaveGame|CreateSaveGameObject "/Game/VRyu/BP_VRyuSaveGame.BP_VRyuSaveGame_C"))
            (Variables|Default|SetSettings _returnvalue_3))))
      (:then_1
        (Variables|Default|SetSettingsLoaded true)))))

(fn PlayManagedSound
  (params (SoundEvent :type E_SoundEvents%20Enum :default "NewEnumerator1") (Location :type Vector) (Pitch :type Float%20%28double-precision%29))
  (Audio|PlaySoundatLocation (.Value (Utilities|Map|Find (Variables|Default|GetSoundMap) SoundEvent)) Location "0, 0, 0" 1.0 Pitch 0.0 0 0 0 0))